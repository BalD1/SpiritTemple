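; BP_MagicalPath is one segment of a glowing path, built as a chain in the editor and lit or unlit segment by segment.
; Editor events spawn the next segment in four directions, rotate the chain's last piece or toggle its straight/curved meshes.
; LitPath and UnlitPath recolor the center material, then propagate recursively with optional delay, handing off to a RelatedIntersection at the end.
; Destroying a segment destroys those after it.
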(event `AddPathEast`
  ;[1 1 1] Editor Events
  (`self.AddPath` (100.0 0.0 0.0)))

(event `AddPathWest`
  ;[1 1 1] Editor Events
  (`self.AddPath` (-100.0 0.0 0.0)))

(event `AddPathSouth`
  ;[1 1 1] Editor Events
  (`self.AddPath` (0.0 100.0 0.0)))

(event `AddPathNorth`
  ;[1 1 1] Editor Events
  (`self.AddPath` (0.0 -100.0 0.0)))

(event `Rotate`
  (bind _relatedpath (`self.RelatedPath`))
  (bind (_returnvalue_roll _returnvalue_pitch _returnvalue_yaw) (`KismetMathLibrary.BreakRotator` (`SceneComponent.K2_GetComponentRotation` (`self.Edges`))))
  ;[1 1 1] Editor Events
  (`/Engine/EditorBlueprintResources/StandardMacros.IsValid` _relatedpath
    (:`Is Valid`
      (`self.Rotate` _relatedpath))
    (:`Is Not Valid`
      (`SceneComponent.K2_SetRelativeRotation` (`self.Edges`) (`KismetMathLibrary.MakeRotator` 0.0 0.0 (+ _returnvalue_yaw 90.0)) false false))))

(event `ChangeLastPath`
  (bind _relatedpath (`self.RelatedPath`))
  ;[1 1 1] Editor Events
  (`/Engine/EditorBlueprintResources/StandardMacros.IsValid` _relatedpath
    (:`Is Valid`
      (`self.ChangeLastPath` _relatedpath))
    (:`Is Not Valid`
      (bind _output_get (set `self.IsCurved` (not (`self.IsCurved`))))
      (if _output_get
        (`StaticMeshComponent.SetStaticMesh` (`self.Edges`) (`self.CurvedEdgesMesh`))
        (`StaticMeshComponent.SetStaticMesh` (`self.Center`) (`self.CurvedCenterMesh`))
        (else
          (`StaticMeshComponent.SetStaticMesh` (`self.Edges`) (`self.StraightEdgesMesh`))
          (`StaticMeshComponent.SetStaticMesh` (`self.Center`) (`self.StraightCenterMesh`)))))))

(event `ChangePath`
  ;[1 1 1] Editor Events
  (bind _output_get (set `self.IsCurved` (not (`self.IsCurved`))))
  (if _output_get
    (`StaticMeshComponent.SetStaticMesh` (`self.Edges`) (`self.CurvedEdgesMesh`))
    (`StaticMeshComponent.SetStaticMesh` (`self.Center`) (`self.CurvedCenterMesh`))
    (else
      (`StaticMeshComponent.SetStaticMesh` (`self.Edges`) (`self.StraightEdgesMesh`))
      (`StaticMeshComponent.SetStaticMesh` (`self.Center`) (`self.StraightCenterMesh`)))))

(event `LitPath`
  (bind _relatedintersection (`self.RelatedIntersection`))
  ;[1 1 1] Liting and unliting the path (recursive)
  (if (not (`self.IsLit`))
    (bind _havedelay (`self.LitBehaviour` true))
    (if _havedelay
      (`KismetSystemLibrary.Delay` (`self.LitDelay`)))
    (if (`KismetSystemLibrary.IsValid` (`self.RelatedPath`))
      (`self.LitPath` (`self.RelatedPath`))
      (else
        (`/Engine/EditorBlueprintResources/StandardMacros.IsValid` _relatedintersection
          (:`Is Valid`
            (`/Game/Blueprints/BP_MagicalPathIntersection.LitPath` _relatedintersection (`self.IsRight`))))))))

(event `UnlitPath`
  (bind _relatedintersection (`self.RelatedIntersection`))
  ;[1 1 1] Liting and unliting the path (recursive)
  (if (`self.IsLit`)
    (bind _havedelay (`self.LitBehaviour` false))
    (if _havedelay
      (`KismetSystemLibrary.Delay` (`self.LitDelay`)))
    (if (`KismetSystemLibrary.IsValid` (`self.RelatedPath`))
      (`self.UnlitPath` (`self.RelatedPath`))
      (else
        (`/Engine/EditorBlueprintResources/StandardMacros.IsValid` _relatedintersection
          (:`Is Valid`
            (`/Game/Blueprints/BP_MagicalPathIntersection.UnlitPath` _relatedintersection (`self.IsRight`))))))))

(event `UpdateVars`
  (bind _relatedpath (`self.RelatedPath`))
  (`/Engine/EditorBlueprintResources/StandardMacros.IsValid` (`self.RelatedPath`)
    (:`Is Valid`
      (set `/Game/Blueprints/BP_MagicalPath.LitDelay` (`self.LitDelay`) _relatedpath)
      (set `/Game/Blueprints/BP_MagicalPath.UnlitColor` (`self.UnlitColor`) _relatedpath)
      (set `/Game/Blueprints/BP_MagicalPath.LitColor1` (`self.LitColor1`) _relatedpath)
      (set `/Game/Blueprints/BP_MagicalPath.LitColor2` (`self.LitColor2`) _relatedpath))))

(event `self.ReceiveDestroyed`
  ;[1 1 1] Destroy children
  (if (`KismetSystemLibrary.IsValid` (`self.RelatedPath`))
    (`self.K2_DestroyActor` (`self.RelatedPath`))))

(fn `AddPath`
  (params (`Added Location` :type "Vector Structure"))
  (bind _relatedpathlocation (`self.RelatedPathLocation`))
  (if (`KismetSystemLibrary.IsValid` (`self.RelatedPath`))
    ;[1 1 1] Check if the new path is in the continuity of the current one
    (if (== _relatedpathlocation `Added Location`)
      ;;[1 1 1] If it is, delegate it to the next one
      (`self.AddPath` (`self.RelatedPath`) _relatedpathlocation)
      (else
        ;;[1 1 1] Else, see if the related path has a path himself, if not DELETE IT
        (`/Engine/EditorBlueprintResources/StandardMacros.IsValid` (`/Game/Blueprints/BP_MagicalPath.RelatedPath` (`self.RelatedPath`))
          (:`Is Not Valid`
            (`self.K2_DestroyActor` (`self.RelatedPath`))
            (bind _returnvalue (`|SpawnActorFromClass` "BP_MagicalPath_C" (`KismetMathLibrary.MakeTransform` (+ `Added Location` (`self.K2_GetActorLocation`))) "Undefined" "OverrideRootScale" null null :!label _label))
            (bind _output_get (set `self.RelatedPath` _returnvalue))
            (set `/Game/Blueprints/BP_MagicalPath.LitDelay` (`self.LitDelay`) _output_get)
            (`SceneComponent.K2_SetRelativeRotation` (`/Game/Blueprints/BP_MagicalPath.Edges` _output_get) (`SceneComponent.RelativeRotation` (`self.Edges`)) false false)
            (set `self.RelatedPathLocation` `Added Location`)))))
    (else
      (goto _label))))

(fn `LitBehaviour`
  (params (LitState :type Boolean))
  (returns (HaveDelay :type Boolean))
  (bind _output_get (set `self.IsLit` LitState))
  (if _output_get
    (`MeshComponent.SetVectorParameterValueOnMaterials` (`self.Center`) "Color" (`KismetMathLibrary.Conv_LinearColorToVector` (`self.LitColor1`)))
    (`MeshComponent.SetVectorParameterValueOnMaterials` (`self.Center`) "Color2" (`KismetMathLibrary.Conv_LinearColorToVector` (`self.LitColor2`)))
    (else
      (`MeshComponent.SetVectorParameterValueOnMaterials` (`self.Center`) "Color" (`KismetMathLibrary.Conv_LinearColorToVector` (`self.UnlitColor`)))
      (`MeshComponent.SetVectorParameterValueOnMaterials` (`self.Center`) "Color2" (`KismetMathLibrary.Conv_LinearColorToVector` (`self.UnlitColor`)))))
  (if (> (`self.LitDelay`) 0.0)
    (return true)
    (else
      (return false))))

(fn `UserConstructionScript`
  (`self.LitBehaviour` (`self.IsLit`))
  (if (and (`KismetSystemLibrary.IsValid` (`self.RelatedPath`)) (`self.IsLit`))
    (`self.LitPath` (`self.RelatedPath`))))