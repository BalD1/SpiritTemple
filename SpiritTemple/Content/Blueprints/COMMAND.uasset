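; COMMAND is a debug cheat blueprint whose custom events are called from the console with `ke * COMMANDNAME`.
; Events tune the first-person character's jump and walk speed, unlock earth, fire and water powers, or print help text.
; Teleport events move the player to a comma-separated coordinate, the WarpZone, or a named point found by substring match in the WarpZone's TeleportationPoints, all through TeleportPlayerTo, which resets rotation to zero.
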(event `HELP`
  (bind _print_duration (`self.Print duration`))
  ;[1 1 1] General
  (`KismetSystemLibrary.PrintString` "PLAYER_JUMP int  : Sets the player's jump height \nPLAYER_SPEED int : Sets the player's speed \n" true true (struct :`G` 0.364583 :`B` 0.058398 :`A` 1.0) _print_duration)
  (`KismetSystemLibrary.PrintString` "UNLOCK_POWER_EARTH       \nUNLOCK_POWER_FIRE              :  Unlocks the given power \nUNLOCK_POWER_WATER   \n" true true (struct :`G` 1.0 :`B` 0.502067 :`A` 1.0) _print_duration) ; Powers
  (`KismetSystemLibrary.PrintString` "TP_HELP                          : Prints every teleportation points names \nTP_AT int,int,int               : Teleport the player to the given location \nTP_WARPZONE               : Teleport the player to the warpzone \nTP_ROOM_ROOMNAME : Teleport the player to the given room \n" true true (struct :`G` 0.964687 :`B` 1.0 :`A` 1.0) _print_duration) ; Teleportation
  (`KismetSystemLibrary.PrintString` "Commands : \nType ke * COMMANDNAME \n" true true (struct :`R` 1.0 :`G` 0.535621 :`A` 1.0) _print_duration) ; Title
)

(event `UNLOCK_POWER_EARTH`
  ;[1 1 1] Powers
  (bind _asfirst_person_character (cast `/Game/FirstPerson/Player/FirstPersonCharacter` (`GameplayStatics.GetPlayerPawn` 0)))
  (`/Game/FirstPerson/Player/FirstPersonCharacter.Unlock Power` _asfirst_person_character 0))

(event `TP_AT`
  (params (NewParam :type String))
  ;[1 1 1] Teleportation
  (bind _outputvector (`self.ParseStringToVector` NewParam))
  (`self.TeleportPlayerTo` _outputvector))

(event `PLAYER_JUMP`
  (params (Height :type "Float (double-precision)"))
  ;[1 1 1] Player
  (bind _asfirst_person_character (cast `/Game/FirstPerson/Player/FirstPersonCharacter` (`GameplayStatics.GetPlayerPawn` 0)))
  (set `CharacterMovementComponent.JumpZVelocity` Height (`Character.CharacterMovement` _asfirst_person_character)))

(event `UNLOCK_POWER_FIRE`
  ;[1 1 1] Powers
  (bind _asfirst_person_character (cast `/Game/FirstPerson/Player/FirstPersonCharacter` (`GameplayStatics.GetPlayerPawn` 0)))
  (`/Game/FirstPerson/Player/FirstPersonCharacter.Unlock Power` _asfirst_person_character 1))

(event `TP_WARPZONE`
  ;[1 1 1] Teleportation
  (`self.TeleportPlayerTo` (`SceneComponent.K2_GetComponentLocation` (`/Game/Blueprints/BP_WarpZone.DefaultSceneRoot` (`self.WarpZone`)))))

(event `PLAYER_SPEED`
  (params (Speed :type "Float (double-precision)"))
  ;[1 1 1] Player
  (bind _asfirst_person_character (cast `/Game/FirstPerson/Player/FirstPersonCharacter` (`GameplayStatics.GetPlayerPawn` 0)))
  (set `CharacterMovementComponent.MaxWalkSpeed` Speed (`Character.CharacterMovement` _asfirst_person_character)))

(event `UNLOCK_POWER_WATER`
  ;[1 1 1] Powers
  (bind _asfirst_person_character (cast `/Game/FirstPerson/Player/FirstPersonCharacter` (`GameplayStatics.GetPlayerPawn` 0)))
  (`/Game/FirstPerson/Player/FirstPersonCharacter.Unlock Power` _asfirst_person_character 2))

(event `TP_HELP`
  ;[1 1 1] Teleportation
  (`KismetSystemLibrary.PrintString` "TP EARTHENTRY \nTP EARTHLABYRINTH \nTP EARTHROOMA \nTP EARTHROOMB \n \nTP WATER \n \nTP FIREENTRY \nTP FIREROOMA \nTP FIREROOMB \n \nTP ENDING" true true (struct :`G` 0.964687 :`B` 1.0 :`A` 1.0) (`self.Print duration`)))

(event `UNLOCK_POWER_ALL`
  ;[1 1 1] Powers
  (bind _asfirst_person_character (cast `/Game/FirstPerson/Player/FirstPersonCharacter` (`GameplayStatics.GetPlayerPawn` 0)))
  (for _index (range 3)
    (`/Game/FirstPerson/Player/FirstPersonCharacter.Unlock Power` _asfirst_person_character _index)))

(event `TP`
  (params (`Point Name` :type String))
  ;[1 1 1] Teleportation
  (bind _point_position (`self.Search TP Point` `Point Name`))
  (`self.TeleportPlayerTo` _point_position))

(fn `ParseStringToVector`
  (params (SourceString :type String))
  (returns (OutputVector :type "Vector Structure"))
  (bind _returnvalue (`KismetStringLibrary.ParseIntoArray` SourceString ","))
  (return (`KismetMathLibrary.MakeVector` (`KismetStringLibrary.Conv_StringToDouble` (`|GetArrayItem` _returnvalue)) (`KismetStringLibrary.Conv_StringToDouble` (`|GetArrayItem` _returnvalue 1)) (`KismetStringLibrary.Conv_StringToDouble` (`|GetArrayItem` _returnvalue 2)))))

(fn `Search TP Point`
  (params (`Searched Point` :type String))
  (returns (`Point Position` :type "Vector Structure"))
  (for _array_element (`/Game/Blueprints/BP_WarpZone.Teleportation Points` (`self.WarpZone`))
    (if (`KismetStringLibrary.Contains` (`KismetSystemLibrary.GetObjectName` _array_element) `Searched Point`)
      (break)))
  (return (`SceneComponent.K2_GetComponentLocation` (`/Game/Blueprints/BP_Teleport.TPPoint` _array_element))))

(fn `TeleportPlayerTo`
  (params (Position :type "Vector Structure"))
  (`self.K2_TeleportTo` :`self` (`GameplayStatics.GetPlayerPawn` 0) :`DestLocation` Position))

(fn `UserConstructionScript`)