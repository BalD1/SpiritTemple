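; BP_EndMapTP is a trigger actor that moves the first-person player into the end-of-map sequence.
; On overlap it disables sprint and jump, stops walking, fades to black, then starts a non-blocking stream load of EndMap.
; It reveals the last chakra stand, spawns its chakra, and teleports the player to TPPoint at walk speed 200.
; After fading back in, it calls HideCharacter, then unlights FirstStep and destroys itself if that step is valid.
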(event `self.Trigger.OnComponentBeginOverlap`
  (params (OverlappedComponent :type "PrimitiveComponent Object Reference") (OtherActor :type "Actor Object Reference") (OtherComp :type "PrimitiveComponent Object Reference") (OtherBodyIndex :type Integer) (bFromSweep :type Boolean) (SweepResult :type "HitResult Structure (by ref)"))
  (bind _firststep (`self.FirstStep`))
  (bind _asfirst_person_character (cast `/Game/FirstPerson/Player/FirstPersonCharacter` OtherActor))
  (bind _outplayer (`self.RestrainPlayer` _asfirst_person_character))
  (`/Game/Blueprints/UI/PlayerUi.FadeToBlack` (`/Game/Blueprints/UI/UiManager.Player Ui` (`/Game/FirstPerson/Player/FirstPersonCharacter.UIManager` _outplayer)) "Forward")
  (`KismetSystemLibrary.Delay` 1.0)
  (`GameplayStatics.LoadStreamLevel` "EndMap" true)
  (`self.SpawnChakra`)
  (`self.K2_TeleportTo` :`self` _outplayer :`DestLocation` (`self.K2_GetActorLocation` (`self.TP Point`)))
  (set `CharacterMovementComponent.MaxWalkSpeed` 200.0 (`Character.CharacterMovement` _outplayer))
  (`KismetSystemLibrary.Delay` 0.5)
  (`/Game/Blueprints/UI/PlayerUi.FadeToBlack` (`/Game/Blueprints/UI/UiManager.Player Ui` (`/Game/FirstPerson/Player/FirstPersonCharacter.UIManager` _outplayer)) "Reverse")
  (`/Game/FirstPerson/Player/FirstPersonCharacter.HideCharacter` _outplayer true)
  (`/Engine/EditorBlueprintResources/StandardMacros.IsValid` _firststep
    (:`Is Valid`
      (`/Game/Blueprints/BP_MagicalStep.UnlitStep` _firststep)
      (`self.K2_DestroyActor`))))

(fn `RestrainPlayer`
  (params (InPlayer :type "/Game/FirstPerson/Player/FirstPersonCharacter Object Reference"))
  (returns (OutPlayer :type "/Game/FirstPerson/Player/FirstPersonCharacter Object Reference"))
  (set `/Game/FirstPerson/Player/FirstPersonCharacter.CanSprint` false InPlayer)
  (set `CharacterMovementComponent.MaxWalkSpeed` 0.0 (`Character.CharacterMovement` InPlayer))
  (set `/Game/FirstPerson/Player/FirstPersonCharacter.CanJumpp` false InPlayer)
  (return InPlayer))

(fn `SpawnChakra`
  (bind _lastchakrastand (`self.LastChakraStand`))
  (`SceneComponent.SetVisibility` (`/Game/Blueprints/Chakras/BP_ChakraBall_Stand.Mesh` _lastchakrastand) true false)
  (`/Game/Blueprints/Chakras/BP_ChakraBall_Stand.SpawnChakra` _lastchakrastand))

(fn `UserConstructionScript`)