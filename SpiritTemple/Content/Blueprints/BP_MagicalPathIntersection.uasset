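; BP_MagicalPathIntersection is a magical path junction that lights its forward path once both incoming sides are lit.
; LitPath and UnlitPath swap the Left or Right mesh material and adjust a shared counter.
; A count of two or more lights the Front mesh and propagates to FrontPath.
; Any decrement immediately unlights Front and propagates the unlit state onward.
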(event `AddCounter`
  (bind _count (`self.Count`))
  (`/Engine/EditorBlueprintResources/StandardMacros.IncrementInt` _count
    (:`  `
      (if (>= _count 2)
        (`PrimitiveComponent.SetMaterial` (`self.Front`) 0 (`self.LitMaterial`))
        (`/Game/Blueprints/BP_MagicalPath.LitPath` (`self.FrontPath`))))))

(event `DecrementeCounter`
  (`/Engine/EditorBlueprintResources/StandardMacros.DecrementInt` (`self.Count`)
    (:`  `
      (`PrimitiveComponent.SetMaterial` (`self.Front`) 0 (`self.UnlitMaterial`))
      (`/Game/Blueprints/BP_MagicalPath.UnlitPath` (`self.FrontPath`)))))

(fn `LitPath`
  (params (Right :type Boolean))
  (if Right
    (`PrimitiveComponent.SetMaterial` (`self.Right`) 0 (`self.LitMaterial`))
    (else
      (`PrimitiveComponent.SetMaterial` (`self.Left`) 0 (`self.LitMaterial`))))
  (`self.AddCounter`))

(fn `UnlitPath`
  (params (Right :type Boolean))
  (if Right
    (`PrimitiveComponent.SetMaterial` (`self.Right`) 0 (`self.UnlitMaterial`))
    (else
      (`PrimitiveComponent.SetMaterial` (`self.Left`) 0 (`self.UnlitMaterial`))))
  (`self.DecrementeCounter`))

(fn `UserConstructionScript`)