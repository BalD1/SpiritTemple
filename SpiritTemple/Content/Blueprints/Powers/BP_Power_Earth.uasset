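; Earth power Blueprint that lets the player punch earth interactable objects.
; PowerAction marks the punch and the player's power as in use, then clears both after the action animation's length, resetting the punch flag on the selected power if it is an Earth power.
; PunchAction runs a short line trace from the player toward camera center and calls HasBeenPunched on any BP_EarthInteractable hit.
; Trigger collision is disabled on BeginPlay.
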(event `self.ReceiveBeginPlay`
  (`parent.ReceiveBeginPlay`)
  (`PrimitiveComponent.SetCollisionEnabled` (`self.Trigger`) "NoCollision"))

(event `self.Power Action`
  (bind _playerref (`self.PlayerRef`))
  (if (not (`self.IsPunching`))
    (set `self.IsPunching` true)
    (set `/Game/FirstPerson/Player/FirstPersonCharacter.PowerIsInUse` true _playerref)
    (bind _returnvalue (`AnimSequenceBase.GetPlayLength` (`/Game/FirstPerson/Player/FirstPersonCharacter.ActionAnim` _playerref)))
    (`KismetSystemLibrary.Delay` _returnvalue)
    (set `/Game/FirstPerson/Player/FirstPersonCharacter.PowerIsInUse` false _playerref)
    (bind _asbp_power_earth (cast `/Game/Blueprints/Powers/BP_Power_Earth` (`/Game/FirstPerson/Player/FirstPersonCharacter.SelectedPower` _playerref)))
    (set `/Game/Blueprints/Powers/BP_Power_Earth.IsPunching` false _asbp_power_earth)))

(event `PunchAction`
  (bind _out_hit (`self.TraceLineFromPlayerToCamCenter` (struct :`R` 0.215861 :`G` 0.116971 :`B` 0.056128 :`A` 1.0) 100.0))
  (bind _asbp_earth_interactable (cast `/Game/Blueprints/Interactables/Earth/BP_EarthInteractable` (`.HitActor` (`GameplayStatics.BreakHitResult` _out_hit))))
  (`/Game/Blueprints/Interactables/Earth/BP_EarthInteractable.HasBeenPunched` _asbp_earth_interactable))

(fn `UserConstructionScript`
  (`parent.UserConstructionScript`))