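; BP_PowerBase is a power Blueprint that fires projectiles for the player.
; FireProjectile loops over the Powers collection on PlayerRef and, for each entry both selected and unlocked, spawns a BP_Projectile.
; Each projectile spawns at the player's FirePoint location, oriented to the first-person camera's world rotation.
; The projectile class is fixed, so it does not vary with the selected power.
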(fn `FireProjectile`
  (bind _playerref (`self.PlayerRef`))
  (for _array_element (`/Game/FirstPerson/Player/FirstPersonCharacter.Powers` (`self.PlayerRef`))
    (if (and (`.IsSelected_5_E7BD257A4D150E636AF12FA84B87782C` (break `/Game/Blueprints/Powers/STRUCT_PlayerPowersInv` _array_element)) (`.IsUnlocked_7_CFA486FE4796F5E69FD31BA3118A5A40` (break `/Game/Blueprints/Powers/STRUCT_PlayerPowersInv` _array_element)))
      (`|SpawnActorFromClass` "/Game/Blueprints/Powers/Projecties/BP_Projectile.BP_Projectile_C" (`KismetMathLibrary.MakeTransform` (`SceneComponent.K2_GetComponentLocation` (`/Game/FirstPerson/Player/FirstPersonCharacter.FirePoint` _playerref)) (`SceneComponent.K2_GetComponentRotation` (`/Game/FirstPerson/Player/FirstPersonCharacter.FirstPersonCamera` _playerref))) "Undefined" "OverrideRootScale" null null))))

(fn `UserConstructionScript`)