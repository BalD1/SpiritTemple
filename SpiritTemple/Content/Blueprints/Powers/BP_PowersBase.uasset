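; Base Blueprint for first-person player powers, which starts inactive and attaches to the hand socket on the player's arms.
; While active, Tick line-traces from the camera out to Range, stores the hit location and passes the hit actor to InteractableInRange.
; That event, UnselectPower and SecondaryPowerAction are empty hooks.
; PowerAction locks the player's PowerIsInUse flag for roughly half the action animation's length.
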(event `self.ReceiveTick`
  (params (DeltaSeconds :type "Float (single-precision)"))
  (if (`self.IsActive`)
    (bind _out_hit (`self.TraceLineFromPlayerToCamCenter` (struct :`R` 1.0 :`B` 0.775802 :`A` 1.0) (`self.Range`)))
    (bind (_bblockinghit _binitialoverlap _time _distance _location _impactpoint _normal _impactnormal _physmat _hitactor) (`GameplayStatics.BreakHitResult` _out_hit))
    (`self.InteractableInRange` _hitactor)
    (set `self.HitLocation` _location)))

(event `InteractableInRange`
  (params (Hit :type "Actor Object Reference")))

(event `UnselectPower`)

(event `self.ReceiveBeginPlay`
  (bind _playerref (`self.PlayerRef`))
  (`self.SetActive` false)
  (`self.K2_AttachToComponent` (`/Game/FirstPerson/Player/FirstPersonCharacter.Arms` _playerref) (`/Game/FirstPerson/Player/FirstPersonCharacter.HandSocketName` _playerref) "KeepRelative" "KeepRelative" "KeepRelative"))

(event `Secondary Power Action`)

(event `Power Action`
  (bind _playerref (`self.PlayerRef`))
  (if (not (`/Game/FirstPerson/Player/FirstPersonCharacter.PowerIsInUse` _playerref))
    (set `/Game/FirstPerson/Player/FirstPersonCharacter.PowerIsInUse` true _playerref)
    (bind _returnvalue (`AnimSequenceBase.GetPlayLength` (`self.ActionAnim`)))
    (`KismetSystemLibrary.Delay` (/ _returnvalue 1.9))
    (set `/Game/FirstPerson/Player/FirstPersonCharacter.PowerIsInUse` false _playerref)))

(fn `SetActive`
  (params (Active :type Boolean))
  (`self.SetActorHiddenInGame` (not Active))
  (`ActorComponent.Activate` (`self.Particles`) true)
  (`self.SetActorEnableCollision` Active))

(fn `TraceLineFromPlayerToCamCenter`
  (params (`Trace Color` :type "LinearColor Structure") (Distance :type "Float (double-precision)" :default -1.0))
  (returns (`Out Hit` :type "HitResult Structure") (`Return Value` :type Boolean))
  (bind _firstpersoncamera (`/Game/FirstPerson/Player/FirstPersonCharacter.FirstPersonCamera` (`self.PlayerRef`)))
  (bind _returnvalue (`SceneComponent.K2_GetComponentLocation` _firstpersoncamera))
  (bind (_outhit _returnvalue_2) (`KismetSystemLibrary.LineTraceSingle` :`Start` _returnvalue :`End` (+ _returnvalue (* (`KismetMathLibrary.GetForwardVector` (`SceneComponent.K2_GetComponentRotation` _firstpersoncamera)) Distance)) :`TraceChannel` "TraceTypeQuery1" :`DrawDebugType` "ForDuration" :`TraceColor` `Trace Color` :`DrawTime` 0.0))
  (return _outhit _returnvalue_2))

(fn `UserConstructionScript`)