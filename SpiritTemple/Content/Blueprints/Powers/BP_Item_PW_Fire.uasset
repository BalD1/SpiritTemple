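; BP_Item_PW_Fire is a pickup item, named for the fire power, that unlocks and equips a player power when its trigger is overlapped.
; On overlap it runs a FirstPersonCharacter cast check, then PowerUnlock, then destroys itself.
; PowerUnlock finds the entry matching SearchedPowerName in the player's Powers array, deselects the current power, marks the match unlocked and selected, and updates SelectedPowerIndex.
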(event `self.Trigger.OnComponentBeginOverlap`
  (params (OverlappedComponent :type "PrimitiveComponent Object Reference") (OtherActor :type "Actor Object Reference") (OtherComp :type "PrimitiveComponent Object Reference") (OtherBodyIndex :type Integer) (bFromSweep :type Boolean) (SweepResult :type "HitResult Structure (by ref)"))
  (`self.OnPlayerCollision` OtherActor)
  (`self.PowerUnlock`)
  (`self.K2_DestroyActor`))

(fn `OnPlayerCollision`
  (params (Other :type "Actor Object Reference"))
  (cast `/Game/FirstPerson/Player/FirstPersonCharacter` Other))

(fn `PowerUnlock`
  (bind _playerref (`self.PlayerRef`))
  (bind _powers (`/Game/FirstPerson/Player/FirstPersonCharacter.Powers` _playerref))
  (for (_array_element _array_index) (`/Game/FirstPerson/Player/FirstPersonCharacter.Powers` (`self.PlayerRef`))
    (if (`|EnumEquality` (break `/Game/Blueprints/Powers/STRUCT_PlayerPowersInv` _array_element) (`self.SearchedPowerName`))
      (setmembers `/Game/Blueprints/Powers/STRUCT_PlayerPowersInv` :`StructRef` (`|GetArrayItem` _powers (`/Game/FirstPerson/Player/FirstPersonCharacter.SelectedPowerIndex` _playerref)) :`IsSelected` false)
      (setmembers `/Game/Blueprints/Powers/STRUCT_PlayerPowersInv` :`StructRef` (`|GetArrayItem` _powers _array_index) :`IsSelected` true :`IsUnlocked` true)
      (set `/Game/FirstPerson/Player/FirstPersonCharacter.SelectedPowerIndex` _array_index (`self.PlayerRef`)))))

(fn `UserConstructionScript`)