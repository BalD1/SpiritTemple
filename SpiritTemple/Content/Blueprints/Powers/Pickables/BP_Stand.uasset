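; BP_Stand is a pedestal actor that spawns an elemental power pickup (Earth, Fire or Water) at its PowerPoint component.
; SpawnPowerByName maps the power name to the matching item Blueprint, and SpawnPickable spawns it at that point's world transform.
; It spawns its configured PowerName on BeginPlay when SpawnAtStart is set, or any named power through the SpawnPower event.
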(event `self.ReceiveBeginPlay`
  (if (`self.SpawnAtStart`)
    (`self.SpawnPowerByName` (`self.PowerName`))))

(event `SpawnPower`
  (params (PowerName :type "/Game/Blueprints/Powers/ENUM_PWnames Enum" :default "NewEnumerator0"))
  (`self.SpawnPowerByName` PowerName))

(fn `Spawn Pickable`
  (params (Item :type "/Game/Blueprints/Powers/Pickables/BP_Pickable_PW Class Reference"))
  (`|SpawnActorFromClass` Item (`SceneComponent.K2_GetComponentToWorld` (`self.PowerPoint`)) "Undefined" "OverrideRootScale" null null))

(fn `SpawnPowerByName`
  (params (Selection :type "/Game/Blueprints/Powers/ENUM_PWnames Enum" :default "NewEnumerator0"))
  (switch `/Game/Blueprints/Powers/ENUM_PWnames` Selection
    (:`NewEnumerator0`
      (`self.Spawn Pickable` "/Game/Blueprints/Powers/Pickables/BP_Item_PW_Earth.BP_Item_PW_Earth_C"))
    (:`NewEnumerator1`
      (`self.Spawn Pickable` "/Game/Blueprints/Powers/Pickables/BP_Item_PW_Fire.BP_Item_PW_Fire_C"))
    (:`NewEnumerator3`
      (`self.Spawn Pickable` "/Game/Blueprints/Powers/Pickables/BP_Item_PW_Water.BP_Item_PW_Water_C"))))

(fn `UserConstructionScript`)