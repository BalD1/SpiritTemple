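; BP_Pickable_PW is a pickable power actor that unlocks a power for the player and then destroys itself.
; Its TriggerUnlock event runs PowerUnlock, which casts player pawn 0 to FirstPersonCharacter and searches its Powers array for the entry named SearchedPowerName.
; The resulting array index is passed to the character's UnlockPower, with no separate handling for a name that is not found.
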(event `TriggerUnlock`
  (`self.PowerUnlock`)
  (`self.K2_DestroyActor`))

(fn `PowerUnlock`
  (bind _asfirst_person_character (cast `/Game/FirstPerson/Player/FirstPersonCharacter` (`GameplayStatics.GetPlayerPawn` 0)))
  ;[1 1 1] Search power in player's inventory
  (for (_array_element _array_index) (`/Game/FirstPerson/Player/FirstPersonCharacter.Powers` _asfirst_person_character)
    (if (`|EnumEquality` (break `/Game/Blueprints/Powers/STRUCT_PlayerPowersInv` _array_element) (`self.SearchedPowerName`))
      (break)))
  (`/Game/FirstPerson/Player/FirstPersonCharacter.Unlock Power` _asfirst_person_character _array_index))

(fn `UserConstructionScript`)