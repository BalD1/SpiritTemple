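; Chakra plate actor that lights up by driving the Radius parameter of a cut-off material on its mesh.
; The construction script picks plate and background materials per chakra, then applies boost, hardness, power, fringe color, optional emissiveness and a min or max starting radius.
; ProgressiveLit animates the radius by a fraction of its maximum over a set time on Tick, while InstantLit adds it immediately, clamped.
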(event `self.ReceiveTick`
  (params (DeltaSeconds :type "Float (single-precision)"))
  ;[1 1 1] Timer
  (if (> (`self.LitTime`) 0.0)
    (set `self.Timer` (+ (`self.Timer`) DeltaSeconds))
    ;[1 1 1] Lerp
    (bind _output_get (set `self.M_Radius` (+ (`self.LastRadius`) (* (* (`self.AlphaGoal`) (/ (`self.Timer`) (`self.LitTime`))) (`self.M_RadiusMax`)))))
    ;[1 1 1] Lit
    (`MeshComponent.SetScalarParameterValueOnMaterials` (`self.Mesh`) "Radius" _output_get)
    ;[1 1 1] Timer end
    (if (>= (`self.Timer`) (`self.LitTime`))
      (set `self.LitTime` 0.0)
      (set `self.Timer` 0.0))))

(event `ProgressiveLit`
  (params (AlphaToAdd :type "Float (double-precision)") (Time :type "Float (double-precision)"))
  ;[1 1 1] Set timer, goal, and radius
  (set `self.AlphaGoal` AlphaToAdd)
  (set `self.LitTime` Time)
  (set `self.Timer` 0.0)
  (set `self.LastRadius` (`self.M_Radius`)))

(event `InstantLit`
  (params (Alpha :type "Float (double-precision)"))
  ;[1 1 1] Lit without lerp
  (bind _output_get (set `self.M_Radius` (`KismetMathLibrary.FClamp` (+ (`self.M_Radius`) (* Alpha (`self.M_RadiusMax`))) 0.0 (`self.M_RadiusMax`))))
  (`MeshComponent.SetScalarParameterValueOnMaterials` (`self.Mesh`) "Radius" _output_get))

(fn `SetMaterials`
  (switch `/Game/Blueprints/Chakras/ENUM_ChakrasNames` (`self.Chakra`)
    (:`NewEnumerator0`
      (`PrimitiveComponent.SetMaterial` (`self.Mesh`) 0 "/Game/Materials/Chakras/Fading/M_CutOff_Material_Muladhara.M_CutOff_Material_Muladhara")
      (`PrimitiveComponent.SetMaterial` (`self.BackgroundPlate`) 0 "/Game/Materials/Chakras/M_Chakra_Muladhara.M_Chakra_Muladhara"))
    (:`NewEnumerator1`
      (`PrimitiveComponent.SetMaterial` (`self.Mesh`) 0 "/Game/Materials/Chakras/Fading/M_CutOff_Material_Swadhistana.M_CutOff_Material_Swadhistana")
      (`PrimitiveComponent.SetMaterial` (`self.BackgroundPlate`) 0 "/Game/Materials/Chakras/M_Chakra_Swadhistana.M_Chakra_Swadhistana"))
    (:`NewEnumerator2`
      (`PrimitiveComponent.SetMaterial` (`self.Mesh`) 0 "/Game/Materials/Chakras/Fading/M_CuttOff_Material_Manipura.M_CuttOff_Material_Manipura")
      (`PrimitiveComponent.SetMaterial` (`self.BackgroundPlate`) 0 "/Game/Materials/Chakras/M_Chakra_Manipura.M_Chakra_Manipura"))
    (:`NewEnumerator3`
      (`PrimitiveComponent.SetMaterial` (`self.Mesh`) 0 "/Game/Materials/Chakras/Fading/M_CuttOff_Material_Anahata.M_CuttOff_Material_Anahata")
      (`PrimitiveComponent.SetMaterial` (`self.BackgroundPlate`) 0 "/Game/Materials/Chakras/M_Chakra_Anahata.M_Chakra_Anahata"))
    (:`NewEnumerator4`
      (`PrimitiveComponent.SetMaterial` (`self.Mesh`) 0 "/Game/Materials/Chakras/Fading/M_CuttOff_Material_Vishuda.M_CuttOff_Material_Vishuda")
      (`PrimitiveComponent.SetMaterial` (`self.BackgroundPlate`) 0 "/Game/Materials/Chakras/M_ChakraVishuda.M_ChakraVishuda"))
    (:`NewEnumerator5`
      (`PrimitiveComponent.SetMaterial` (`self.Mesh`) 0 "/Game/Materials/Chakras/Fading/M_CuttOff_Material_Ajna.M_CuttOff_Material_Ajna")
      (`PrimitiveComponent.SetMaterial` (`self.BackgroundPlate`) 0 "/Game/Materials/Chakras/M_ChakraAjna.M_ChakraAjna"))
    (:`NewEnumerator6`
      (`PrimitiveComponent.SetMaterial` (`self.Mesh`) 0 "/Game/Materials/Chakras/Fading/M_CuttOff_Material_Sahasrara.M_CuttOff_Material_Sahasrara")
      (`PrimitiveComponent.SetMaterial` (`self.BackgroundPlate`) 0 "/Game/Materials/Chakras/M_Chakra_Sahasrara.M_Chakra_Sahasrara")))
  (`MeshComponent.SetVectorParameterValueOnMaterials` (`self.BackgroundPlate`) "Color" (0.0 0.0 0.0)))

(fn `UserConstructionScript`
  (`self.SetMaterials`)
  (`MeshComponent.SetScalarParameterValueOnMaterials` (`self.Mesh`) "Boost" (`self.M_Boost`))
  (`MeshComponent.SetScalarParameterValueOnMaterials` (`self.Mesh`) "Hardness" (`self.M_Hardness`))
  (`MeshComponent.SetScalarParameterValueOnMaterials` (`self.Mesh`) "Power" (`self.M_Power`))
  (if (`self.M_RadiusAtMin`)
    (`MeshComponent.SetScalarParameterValueOnMaterials` (`self.Mesh`) "Radius" (`self.M_RadiusMin`))
    (set `self.M_Radius` (`self.M_RadiusMin`))
    (else
      (`MeshComponent.SetScalarParameterValueOnMaterials` (`self.Mesh`) "Radius" (`self.M_RadiusMax`))
      (set `self.M_Radius` (`self.M_RadiusMax`))))
  (`MeshComponent.SetVectorParameterValueOnMaterials` (`self.Mesh`) "FringeColor" (`KismetMathLibrary.Conv_LinearColorToVector` (`self.M_CutOffColor`)))
  (if (`self.UseEmissivness`)
    (`MeshComponent.SetScalarParameterValueOnMaterials` (`self.Mesh`) "UseEmissivness" 1.0)
    (`MeshComponent.SetScalarParameterValueOnMaterials` (`self.Mesh`) "Emissivness" (`self.EmissivnessValue`))
    (else
      (`MeshComponent.SetScalarParameterValueOnMaterials` (`self.Mesh`) "UseEmissivness" -1.0))))