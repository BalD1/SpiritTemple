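; BP_PlateBase is a base plate actor that switches between lit and unlit states.
; UpdateState flips IsLit and calls UpdateLitState, which also runs at BeginPlay to apply the initial state.
; UpdateLitState sets the Color vector parameter on the Plate's materials to LitColor when lit, or to black when unlit.
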(event `self.ReceiveBeginPlay`
  (`self.UpdateLitState`))

(event `UpdateState`
  (set `self.IsLit` (not (`self.IsLit`)))
  (`self.UpdateLitState`))

(fn `UpdateLitState`
  (if (`self.IsLit`)
    (`MeshComponent.SetVectorParameterValueOnMaterials` (`self.Plate`) "Color" (`KismetMathLibrary.Conv_LinearColorToVector` (`self.LitColor`)))
    (else
      (`MeshComponent.SetVectorParameterValueOnMaterials` (`self.Plate`) "Color" (0.0 0.0 0.0)))))

(fn `UserConstructionScript`)