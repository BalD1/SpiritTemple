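; BP_FadingPlate is a one-shot plate whose material Radius animates toward its maximum when the first-person character overlaps its trigger.
; The construction script applies the Chakra material and its tuning parameters, starting Radius at either minimum or maximum.
; On overlap, the trigger disables its collision and plays a timeline that feeds the current radius back into each Lerp, compounding the approach to the maximum.
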(event `self.Trigger.OnComponentBeginOverlap`
  (params (OverlappedComponent :type "PrimitiveComponent Object Reference") (OtherActor :type "Actor Object Reference") (OtherComp :type "PrimitiveComponent Object Reference") (OtherBodyIndex :type Integer) (bFromSweep :type Boolean) (SweepResult :type "HitResult Structure (by ref)"))
  (cast `/Game/FirstPerson/Player/FirstPersonCharacter` OtherActor)
  (`PrimitiveComponent.SetCollisionEnabled` (`self.Trigger`) "NoCollision")
  (bind (_direction _track) (`Timeline|Timeline` :!via `PlayFromStart`)
    (:`Update`
      (bind _output_get (set `self.M_Radius` (`KismetMathLibrary.Lerp` (`self.M_Radius`) (`self.M_RadiusMax`) _track)))
      (`MeshComponent.SetScalarParameterValueOnMaterials` (`self.Mesh`) "Radius" _output_get))))

(fn `UserConstructionScript`
  (`PrimitiveComponent.SetMaterial` (`self.Mesh`) 0 (`self.Chakra`))
  (`MeshComponent.SetScalarParameterValueOnMaterials` (`self.Mesh`) "Boost" (`self.M_Boost`))
  (`MeshComponent.SetScalarParameterValueOnMaterials` (`self.Mesh`) "Hardness" (`self.M_Hardness`))
  (`MeshComponent.SetScalarParameterValueOnMaterials` (`self.Mesh`) "Power" (`self.M_Power`))
  (if (`self.M_RadiusAtMin`)
    (`MeshComponent.SetScalarParameterValueOnMaterials` (`self.Mesh`) "Radius" (`self.M_RadiusMin`))
    (set `self.M_Radius` (`self.M_RadiusMin`))
    (else
      (`MeshComponent.SetScalarParameterValueOnMaterials` (`self.Mesh`) "Radius" (`self.M_RadiusMax`))
      (set `self.M_Radius` (`self.M_RadiusMax`))))
  (`MeshComponent.SetVectorParameterValueOnMaterials` (`self.Mesh`) "FringeColor" (`KismetMathLibrary.Conv_LinearColorToVector` (`self.M_CutOffColor`))))