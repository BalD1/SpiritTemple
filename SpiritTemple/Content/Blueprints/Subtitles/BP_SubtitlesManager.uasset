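; BP_SubtitlesManager shows subtitles from a data table by row name, with optional 2D sound.
; It drives UIManager to display each row's text for its display time, then hides it.
; Requests arriving meanwhile queue in RowsQ and play in order, gated by ShowNextRow.
; A missing row prints the available names and leaves that gate closed, so later requests only queue.
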(event `ShowSubtitles`
  (params (RowName :type Name))
  (bind _rowsq (`self.RowsQ`))
  (bind _uimanager (`self.UIManager`))
  (bind _uimanager_2 (`self.UIManager`))
  (if (`self.ShowNextRow`)
    (set `self.ShowNextRow` false)
    (bind _returnvalue (`|GetDataTableRow` (`self.SubtitlesList`) RowName)
      (:`then`
        (`/Game/Blueprints/UI/UiManager.SetSubtitlesVisibility` _uimanager_2 "SelfHitTestInvisible")
        (bind (_subtitletext _subtitlesound _displaytime) (break `/Game/Blueprints/Subtitles/STRUCT_Subtitles` _returnvalue))
        (`/Game/Blueprints/UI/UiManager.SetSubtitlesText` _uimanager_2 _subtitletext)
        (`/Engine/EditorBlueprintResources/StandardMacros.IsValid` _subtitlesound
          (:`Is Valid`
            (`GameplayStatics.PlaySound2D` _subtitlesound 1.0 1.0 0.0 null null))
          (:`Is Not Valid`
            _))
        (`KismetSystemLibrary.Delay` _displaytime)
        (`/Game/Blueprints/UI/UiManager.SetSubtitlesVisibility` _uimanager "Hidden")
        (`/Game/Blueprints/UI/UiManager.SetSubtitlesText` _uimanager "")
        (set `self.ShowNextRow` true)
        (if (> (`KismetArrayLibrary.Array_Length` (`self.RowsQ`)) 0)
          (`self.ShowSubtitles` (`|GetArrayItem` _rowsq))
          (`KismetArrayLibrary.Array_Remove` _rowsq)))
      (:`RowNotFound`
        (bind _outrownames (`DataTableFunctionLibrary.GetDataTableRowNames` (`self.SubtitlesList`)))
        (for _array_element _outrownames
          (`KismetSystemLibrary.PrintString` (`KismetStringLibrary.Conv_NameToString` _array_element) true true (struct :`R` 1.0 :`B` 0.021536 :`A` 1.0) 15.0))
        (`KismetSystemLibrary.PrintString` (`KismetStringLibrary.Concat_StrStr` (`KismetStringLibrary.Conv_NameToString` RowName) " Not found in DATA_Subtitles. Names are : ") true true (struct :`R` 1.0 :`B` 0.021536 :`A` 1.0) 15.0)))
    (else
      (`KismetArrayLibrary.Array_Add` (`self.RowsQ`) RowName))))

(fn `UserConstructionScript`)