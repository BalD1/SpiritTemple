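; BP_SubtitlesTrigger is a one-shot trigger actor that sends subtitle row names to the FirstPersonCharacter.
; An overlap on its Trigger component or a ForceTrigger event, which uses the player pawn, runs AddToSubtitles.
; That function passes each RowName entry to SetSubtitles and calls DestroyActor inside the loop.
; The construction script enables query-only collision when IsTriggerable is set, otherwise disables it, leaving ForceTrigger as the way to fire it.
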(event `ForceTrigger`
  (`self.AddToSubtitles` (`GameplayStatics.GetPlayerPawn` 0)))

(event `self.Trigger.OnComponentBeginOverlap`
  (params (OverlappedComponent :type "PrimitiveComponent Object Reference") (OtherActor :type "Actor Object Reference") (OtherComp :type "PrimitiveComponent Object Reference") (OtherBodyIndex :type Integer) (bFromSweep :type Boolean) (SweepResult :type "HitResult Structure (by ref)"))
  (`self.AddToSubtitles` OtherActor))

(fn `AddToSubtitles`
  (params (Object :type "Object Object Reference"))
  (bind _asfirst_person_character (cast `/Game/FirstPerson/Player/FirstPersonCharacter` Object))
  (for _array_element (`self.RowName`)
    (`/Game/FirstPerson/Player/FirstPersonCharacter.SetSubtitles` _asfirst_person_character _array_element)
    (`self.K2_DestroyActor`)))

(fn `UserConstructionScript`
  (if (`self.IsTriggerable`)
    (`PrimitiveComponent.SetCollisionEnabled` (`self.Trigger`) "QueryOnly")
    (else
      (`PrimitiveComponent.SetCollisionEnabled` (`self.Trigger`) "NoCollision"))))