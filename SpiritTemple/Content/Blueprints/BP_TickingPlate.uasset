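; BP_TickingPlate is a plate actor whose LitPlate material shows a radius-based effect with a colored fringe.
; The construction script pushes boost, hardness, power and fringe color to the material, starting the radius at its min or max by flag.
; It applies an optional material override after setting those parameters.
; UpdateRadius stores a new minimum radius and pushes it straight to the material, leaving the current-radius variable untouched.
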(event `UpdateRadius`
  (params (NewRadius :type "Float (double-precision)"))
  (bind _output_get (set `self.M_RadiusMin` NewRadius))
  (`MeshComponent.SetScalarParameterValueOnMaterials` (`self.LitPlate`) "Radius" _output_get))

(fn `UserConstructionScript`
  (bind _material (`self.Material`))
  (`MeshComponent.SetScalarParameterValueOnMaterials` (`self.LitPlate`) "Boost" (`self.M_Boost`))
  (`MeshComponent.SetScalarParameterValueOnMaterials` (`self.LitPlate`) "Hardness" (`self.M_Hardness`))
  (`MeshComponent.SetScalarParameterValueOnMaterials` (`self.LitPlate`) "Power" (`self.M_Power`))
  (if (`self.M_RadiusAtMin`)
    (`MeshComponent.SetScalarParameterValueOnMaterials` (`self.LitPlate`) "Radius" (`self.M_RadiusMin`))
    (set `self.M_Radius` (`self.M_RadiusMin`))
    (else
      (`MeshComponent.SetScalarParameterValueOnMaterials` (`self.LitPlate`) "Radius" (`self.M_RadiusMax`))
      (set `self.M_Radius` (`self.M_RadiusMax`))))
  (`MeshComponent.SetVectorParameterValueOnMaterials` (`self.LitPlate`) "FringeColor" (`KismetMathLibrary.Conv_LinearColorToVector` (`self.M_CutOffColor`)))
  (`/Engine/EditorBlueprintResources/StandardMacros.IsValid` _material
    (:`Is Valid`
      (`PrimitiveComponent.SetMaterial` (`self.LitPlate`) 0 _material))))