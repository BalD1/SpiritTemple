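; Interactable actor, apparently a base class, that lets the first-person player trigger an interaction with the InteractWithActor input.
; UpdateInteractPrompt stores whether interaction is allowed, notifies FirstPersonCharacter through CanInteractEvent, then enables the actor's input or calls DisableInput on the player controller.
; Pressing the input while interaction is allowed fires InteractEvent, which is left empty here as a hook for specific behavior.
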(event `self.ReceiveBeginPlay`)

(event `InputAction|InteractWithActor` :consume false
  (params (Key :type "Key Structure"))
  (:`Pressed`
    (if (`self.CanBeInteractedWith`)
      (`self.InteractEvent`))))

(event `UpdateInteractPrompt`
  (params (NewCanInteract :type Boolean))
  (bind _returnvalue (`GameplayStatics.GetPlayerController` 0))
  (set `self.CanBeInteractedWith` NewCanInteract)
  (bind _asfirst_person_character (cast `/Game/FirstPerson/Player/FirstPersonCharacter` (`GameplayStatics.GetPlayerPawn` 0)))
  (`/Game/FirstPerson/Player/FirstPersonCharacter.CanInteractEvent` _asfirst_person_character NewCanInteract)
  (if NewCanInteract
    (`self.EnableInput` _returnvalue)
    (else
      (`self.DisableInput` _returnvalue null))))

(event `InteractEvent`)

(fn `UserConstructionScript`)