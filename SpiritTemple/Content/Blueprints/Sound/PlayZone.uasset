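; PlayZone is a trigger-zone actor that plays the birds audio event through AudioManager while the player pawn is inside its Box.
; Begin overlap starts the event with the current Volume value and sets a flag; end overlap clears it and stops the event.
; While flagged, Tick sets Volume to the player's absolute X-axis distance from the actor's root and prints it, without sending updates to AudioManager.
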(event `self.ReceiveTick`
  (params (DeltaSeconds :type "Float (single-precision)"))
  (bind _returnvalue_x (`KismetMathLibrary.BreakVector` (`SceneComponent.K2_GetComponentLocation` (`self.DefaultSceneRoot`))))
  (bind _returnvalue_x_2 (`KismetMathLibrary.BreakVector` (`self.K2_GetActorLocation` (`GameplayStatics.GetPlayerPawn` 0))))
  (if (`self.flag`)
    (bind _output_get (set `self.volume` (`KismetMathLibrary.Abs` (- _returnvalue_x _returnvalue_x_2))))
    (`KismetSystemLibrary.PrintString` (`KismetStringLibrary.Conv_DoubleToString` _output_get))))

(event `self.Box.OnComponentBeginOverlap`
  (params (OverlappedComponent :type "PrimitiveComponent Object Reference") (OtherActor :type "Actor Object Reference") (OtherComp :type "PrimitiveComponent Object Reference") (OtherBodyIndex :type Integer) (bFromSweep :type Boolean) (SweepResult :type "HitResult Structure (by ref)"))
  (if (== OtherActor (`GameplayStatics.GetPlayerPawn` 0))
    (set `self.flag` true)
    (`/Game/Blueprints/Sound/AudioManager.PlayBirbs_Event` (`self.AudioManager`) (`self.volume`))))

(event `self.Box.OnComponentEndOverlap`
  (params (OverlappedComponent :type "PrimitiveComponent Object Reference") (OtherActor :type "Actor Object Reference") (OtherComp :type "PrimitiveComponent Object Reference") (OtherBodyIndex :type Integer))
  (if (== (`GameplayStatics.GetPlayerPawn` 0) OtherActor)
    (set `self.flag` false)
    (`/Game/Blueprints/Sound/AudioManager.StopBirbs_Event` (`self.AudioManager`))))

(fn `UserConstructionScript`)