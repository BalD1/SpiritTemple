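; AudioManager is an actor Blueprint that plays footstep ("Pas") and bird ("Birbs") sounds at the player pawn's location.
; Custom events fire the one-shot Pas sound or spawn the Birbs sound, whose stop event destroys the spawned audio component.
; The C key triggers Pas playback directly, while nothing in this graph calls the Birbs events.
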(event `self.ReceiveTick`
  (params (DeltaSeconds :type "Float (single-precision)")))

(event `Key|C` :consume false
  (params (Key :type "Key Structure"))
  (:`Pressed`
    (`self.PlayPas_Event`)))

(event `PlayPas_Event`
  (`GameplayStatics.PlaySoundAtLocation` (`self.pas`) (`self.K2_GetActorLocation` (`GameplayStatics.GetPlayerPawn` 0)) (struct) 1.0 1.0 0.0 null null null))

(event `PlayBirbs_Event`
  (bind _returnvalue (`GameplayStatics.SpawnSoundAtLocation` (`self.birbs`) (`self.K2_GetActorLocation` (`GameplayStatics.GetPlayerPawn` 0)) (struct) 1.0 1.0 0.0 null null)))

(event `StopBirbs_Event`
  (`ActorComponent.K2_DestroyComponent` (stale `PlayBirbs_Event` _returnvalue)))

(fn `UserConstructionScript`)