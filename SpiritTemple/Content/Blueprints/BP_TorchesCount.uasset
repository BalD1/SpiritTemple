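; BP_TorchesCount is a puzzle tracker that opens a linked door once all of its related torches are lit.
; On BeginPlay it counts the torches in RelatedTorches and registers itself as each one's RelatedCount, giving them a back-reference.
; Each LitTorch event decrements UnlitTorches and calls OpenDoorEvent on RelatedDoor when the count reaches zero.
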(event `self.ReceiveBeginPlay`
  (bind _relatedtorches (`self.RelatedTorches`))
  (set `self.UnlitTorches` (`KismetArrayLibrary.Array_Length` _relatedtorches))
  (for _array_element _relatedtorches
    (set `/Game/Blueprints/BP_Torch.RelatedCount` self _array_element)))

(event `LitTorch`
  (set `self.UnlitTorches` (- (`self.UnlitTorches`) 1))
  (if (== (`self.UnlitTorches`) 0)
    (`/Game/Blueprints/BP_door.openDoor_Event` (`self.RelatedDoor`))))

(fn `UserConstructionScript`)