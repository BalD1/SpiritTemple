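; BP_ReturnToFresco is an interactable that returns the player to the Fresco.
; Its Box overlap events toggle an "E" interact prompt for the player pawn.
; InteractEvent fades the camera out, waits for the fade, moves the pawn, then fades back in.
; The move adds FrescoTP as a relative world offset rather than setting an absolute destination.
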(event `self.Box.OnComponentBeginOverlap`
  (params (OverlappedComponent :type "PrimitiveComponent Object Reference") (OtherActor :type "Actor Object Reference") (OtherComp :type "PrimitiveComponent Object Reference") (OtherBodyIndex :type Integer) (bFromSweep :type Boolean) (SweepResult :type "HitResult Structure (by ref)"))
  (if (== OtherActor (`GameplayStatics.GetPlayerPawn` 0))
    (`self.UpdateInteractPrompt` true "Press \"E\" to return to the Fresco")))

(event `self.Box.OnComponentEndOverlap`
  (params (OverlappedComponent :type "PrimitiveComponent Object Reference") (OtherActor :type "Actor Object Reference") (OtherComp :type "PrimitiveComponent Object Reference") (OtherBodyIndex :type Integer))
  (if (== OtherActor (`GameplayStatics.GetPlayerPawn` 0))
    (`self.UpdateInteractPrompt` false "Press \"E\" to return to the Fresco")))

(event `self.InteractEvent`
  (`PlayerCameraManager.StartCameraFade` :`self` (`PlayerController.PlayerCameraManager` (`GameplayStatics.GetPlayerController` 0)) :`ToAlpha` 1.0 :`Duration` 1.0 :`bHoldWhenFinished` true)
  (`KismetSystemLibrary.Delay` 1.0)
  (`self.K2_AddActorWorldOffset` (`GameplayStatics.GetPlayerPawn` 0) (`self.FrescoTP`) false false)
  (`PlayerCameraManager.StartCameraFade` :`self` (`PlayerController.PlayerCameraManager` (`GameplayStatics.GetPlayerController` 0)) :`FromAlpha` 1.0 :`Duration` 1.0 :`bHoldWhenFinished` true))

(fn `UserConstructionScript`
  (`parent.UserConstructionScript`))