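; A cinematic camera actor that plays a short cutscene view when its CallCutscene event fires.
; It blends the player's view to itself, waits for the view time plus a door wait time, then blends back to the pawn.
; During the shot, the CutsceneCamera function blocks move and look input and hides the first-person character, and jumping is disabled until the return blend finishes.
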(event `CallCutscene`
  (bind _asfirst_person_character (cast `/Game/FirstPerson/Player/FirstPersonCharacter` (`GameplayStatics.GetPlayerPawn` 0)))
  (set `/Game/FirstPerson/Player/FirstPersonCharacter.CanJumpp` false _asfirst_person_character)
  (`PlayerController.SetViewTargetWithBlend` (`GameplayStatics.GetPlayerController` 0) self (`self.Blend Time`) "VTBlend_Linear" 0.0 false)
  (`self.Cutscene Camera` true)
  (`KismetSystemLibrary.Delay` (+ (`self.View Time`) (`self.DoorWaitTime`)))
  (`PlayerController.SetViewTargetWithBlend` (`GameplayStatics.GetPlayerController` 0) (`GameplayStatics.GetPlayerPawn` 0) (`self.Blend Time`) "VTBlend_Linear" 0.0 false)
  (`KismetSystemLibrary.Delay` (`self.Blend Time`))
  (`self.Cutscene Camera` false)
  (bind _asfirst_person_character_2 (cast `/Game/FirstPerson/Player/FirstPersonCharacter` (`GameplayStatics.GetPlayerPawn` 0)))
  (set `/Game/FirstPerson/Player/FirstPersonCharacter.CanJumpp` true _asfirst_person_character_2))

(fn `Cutscene Camera`
  (params (CutsceneCamera :type Boolean))
  (bind _returnvalue (`GameplayStatics.GetPlayerController` 0))
  (`Controller.SetIgnoreMoveInput` _returnvalue CutsceneCamera)
  (`Controller.SetIgnoreLookInput` _returnvalue CutsceneCamera)
  (bind _asfirst_person_character (cast `/Game/FirstPerson/Player/FirstPersonCharacter` (`GameplayStatics.GetPlayerCharacter` 0)))
  (`/Game/FirstPerson/Player/FirstPersonCharacter.HideCharacter` _asfirst_person_character CutsceneCamera))

(fn `UserConstructionScript`)