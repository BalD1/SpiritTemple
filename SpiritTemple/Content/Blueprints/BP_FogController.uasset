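; Fog controller actor that shows or hides the component of a referenced fog object.
; An EnableFog event sets visibility directly, and a trigger calls it to flip the current state each time a FirstPersonCharacter begins overlapping.
; The construction script uses IsTriggerable to give the trigger query-only collision or disable its collision entirely.
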(event `EnableFog`
  (params (State :type Boolean))
  (`SceneComponent.SetVisibility` (`ExponentialHeightFog.Component` (`self.Fog`)) State false))

(event `self.Trigger.OnComponentBeginOverlap`
  (params (OverlappedComponent :type "PrimitiveComponent Object Reference") (OtherActor :type "Actor Object Reference") (OtherComp :type "PrimitiveComponent Object Reference") (OtherBodyIndex :type Integer) (bFromSweep :type Boolean) (SweepResult :type "HitResult Structure (by ref)"))
  (cast `/Game/FirstPerson/Player/FirstPersonCharacter` OtherActor)
  (`self.EnableFog` (not (`SceneComponent.IsVisible` (`ExponentialHeightFog.Component` (`self.Fog`))))))

(fn `UserConstructionScript`
  (bind _trigger (`self.Trigger`))
  (if (`self.IsTriggerable`)
    (`PrimitiveComponent.SetCollisionEnabled` _trigger "QueryOnly")
    (else
      (`PrimitiveComponent.SetCollisionEnabled` _trigger "NoCollision"))))