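; BP_ChakrasBar is a bar actor with a material-driven glow that can be lit up through the LitBar event.
; The construction script pushes boost, hardness, power, color and fringe color to the static mesh's materials and starts Radius at min or max according to MRadiusAtMin.
; LitBar plays a timeline that grows Radius toward its max, lerping from the current value each update rather than from a fixed start.
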(event `LitBar`
  (bind (_direction _track) (`Timeline|Timeline` :!via `PlayFromStart`)
    (:`Update`
      (bind _output_get (set `self.M_Radius` (`KismetMathLibrary.Lerp` (`self.M_Radius`) (`self.M_RadiusMax`) _track)))
      (`MeshComponent.SetScalarParameterValueOnMaterials` (`self.StaticMesh`) "Radius" _output_get))))

(fn `UserConstructionScript`
  (`MeshComponent.SetScalarParameterValueOnMaterials` (`self.StaticMesh`) "Boost" (`self.M_Boost`))
  (`MeshComponent.SetScalarParameterValueOnMaterials` (`self.StaticMesh`) "Hardness" (`self.M_Hardness`))
  (`MeshComponent.SetScalarParameterValueOnMaterials` (`self.StaticMesh`) "Power" (`self.M_Power`))
  (if (`self.M_RadiusAtMin`)
    (`MeshComponent.SetScalarParameterValueOnMaterials` (`self.StaticMesh`) "Radius" (`self.M_RadiusMin`))
    (set `self.M_Radius` (`self.M_RadiusMin`))
    (else
      (`MeshComponent.SetScalarParameterValueOnMaterials` (`self.StaticMesh`) "Radius" (`self.M_RadiusMax`))
      (set `self.M_Radius` (`self.M_RadiusMax`))))
  (`MeshComponent.SetVectorParameterValueOnMaterials` (`self.StaticMesh`) "Color" (`KismetMathLibrary.Conv_LinearColorToVector` (`self.M_GeneralColor`)))
  (`MeshComponent.SetVectorParameterValueOnMaterials` (`self.StaticMesh`) "FringeColor" (`KismetMathLibrary.Conv_LinearColorToVector` (`self.M_CutOffColor`))))