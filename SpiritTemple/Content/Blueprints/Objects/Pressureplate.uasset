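; Pressure plate that reacts when a BP_GrabbableCrate enters or leaves it, optionally disabling the crate's placement if KeepCrate is set.
; Entering triggers the first valid target: opens SpeDoor or KeyDoor and lights MagicalPath, or else closes the HoleInWall.
; Leaving only unlights the path for SpeDoor (its close call is unwired), calls KeyDoor's open event again, or reopens the hole.
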(event `self.ReceiveActorBeginOverlap`
  (params (OtherActor :type "Actor Object Reference"))
  (bind _keydoor (`self.KeyDoor`))
  (bind _openwall (`self.OpenWall`))
  (bind _magicalpath (`self.MagicalPath`))
  (bind _asbp_grabbable_crate (cast `/Game/Blueprints/Interactables/Water/BP_GrabbableCrate` OtherActor))
  (if (`self.KeepCrate`)
    (`/Game/Blueprints/Interactables/Water/BP_GrabbableCrate.SetCanPlace` _asbp_grabbable_crate false))
  (cast `/Game/Blueprints/Objects/SpeDoor` (`self.SpeDoor`)
    (:`then`
      (`/Game/Blueprints/Objects/SpeDoor.openDoorSecond_Event` (`self.SpeDoor`))
      (`/Engine/EditorBlueprintResources/StandardMacros.IsValid` _magicalpath :!label _label
        (:`Is Valid`
          (`/Game/Blueprints/BP_MagicalPath.LitPath` _magicalpath))))
    (:`CastFailed`
      (cast `/Game/Blueprints/Objects/KeyDoor` _keydoor
        (:`then`
          (`/Game/Blueprints/Objects/KeyDoor.openDoor_Event` _keydoor)
          (goto _label))
        (:`CastFailed`
          (cast `/Game/Blueprints/Objects/HoleInWall` _openwall)
          (`/Game/Blueprints/Objects/HoleInWall.Close_Event` _openwall))))))

(event `self.ReceiveActorEndOverlap`
  (params (OtherActor :type "Actor Object Reference"))
  (bind _keydoor (`self.KeyDoor`))
  (bind _openwall (`self.OpenWall`))
  (bind _magicalpath (`self.MagicalPath`))
  (cast `/Game/Blueprints/Interactables/Water/BP_GrabbableCrate` OtherActor)
  (cast `/Game/Blueprints/Objects/SpeDoor` (`self.SpeDoor`)
    (:`then`
      (`/Engine/EditorBlueprintResources/StandardMacros.IsValid` _magicalpath
        (:`Is Valid`
          (`/Game/Blueprints/BP_MagicalPath.UnlitPath` _magicalpath))))
    (:`CastFailed`
      (cast `/Game/Blueprints/Objects/KeyDoor` _keydoor
        (:`then`
          (`/Game/Blueprints/Objects/KeyDoor.openDoor_Event` _keydoor))
        (:`CastFailed`
          (cast `/Game/Blueprints/Objects/HoleInWall` _openwall)
          (`/Game/Blueprints/Objects/HoleInWall.Open_Event` _openwall))))))

(fn `UserConstructionScript`)