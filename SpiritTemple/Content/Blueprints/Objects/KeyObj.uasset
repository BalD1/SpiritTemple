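; KeyObj is a physics object actor, named as a key, that the player picks up on contact and carries.
; A Cube hit by the player pawn sets Flag, disables gravity and prints a debug string.
; While Flag is set, Tick calls Take to reposition the actor in front of the pawn without sweeping.
; Pressing E clears Flag and restores gravity, dropping it.
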(event `self.ReceiveTick`
  (params (DeltaSeconds :type "Float (single-precision)"))
  (if (`self.flag`)
    (`self.Take`)))

(event `self.Cube.OnComponentHit`
  (params (HitComponent :type "PrimitiveComponent Object Reference") (OtherActor :type "Actor Object Reference") (OtherComp :type "PrimitiveComponent Object Reference") (NormalImpulse :type "Vector Structure") (Hit :type "HitResult Structure (by ref)"))
  (if (`self.flag`)
    _
    (elif (== OtherActor (`GameplayStatics.GetPlayerPawn` 0))
      (set `self.flag` true)
      (`PrimitiveComponent.SetEnableGravity` (`self.Cube`) false)
      (`KismetSystemLibrary.PrintString` "b"))))

(event `Key|E` :consume false
  (params (Key :type "Key Structure"))
  (:`Pressed`
    (set `self.flag` false)
    (`PrimitiveComponent.SetEnableGravity` (`self.Cube`) true)))

(fn `Take`
  (bind _returnvalue (`GameplayStatics.GetPlayerPawn` 0))
  (`self.K2_SetActorLocation` (+ (`self.K2_GetActorLocation` _returnvalue) (* (`self.GetActorForwardVector` _returnvalue) 200.0))))

(fn `UserConstructionScript`)