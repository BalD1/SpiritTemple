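; Lever actor that opens a linked Door or Openwall when the player pawn hits its mesh.
; The hit handler rotates the mesh with MoveComponentTo, sets a flag and fires the target's open event, with Door taking priority over Openwall.
; The flag makes it single-use once a valid target is triggered.
; A French note suggests pairing it with the water power, which this logic does not check.
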(event `self.StaticMesh.OnComponentHit`
  (params (HitComponent :type "PrimitiveComponent Object Reference") (OtherActor :type "Actor Object Reference") (OtherComp :type "PrimitiveComponent Object Reference") (NormalImpulse :type "Vector Structure") (Hit :type "HitResult Structure (by ref)"))
  ;[1 1 1] mettre avec le pouvoir d'eau
  (if (`self.flag`)
    _
    (elif (== OtherActor (`GameplayStatics.GetPlayerPawn` 0))
      (`/Engine/EditorBlueprintResources/StandardMacros.IsValid` (`self.door`)
        (:`Is Valid`
          (`KismetSystemLibrary.MoveComponentTo` (`self.StaticMesh`) (0.0 0.0 0.0) (struct :`Pitch` -45.0))
          (set `self.flag` true)
          (`/Game/Blueprints/Objects/SpeDoor.openDoor_Event` (`self.door`)))
        (:`Is Not Valid`
          (`/Engine/EditorBlueprintResources/StandardMacros.IsValid` (`self.openwall`)
            (:`Is Valid`
              (`KismetSystemLibrary.MoveComponentTo` (`self.StaticMesh`) (0.0 0.0 0.0) (struct :`Pitch` -45.0))
              (set `self.flag` true)
              (`/Game/Blueprints/Objects/HoleInWall.Open_Event` (`self.openwall`)))))))))

(fn `UserConstructionScript`)