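; HoleInWall is a wall opening whose static mesh rises when the player's pawn hits the HoleInWall component.
; Open and close events shift the mesh up and down by a fixed relative offset, instantly and without sweep.
; A boolean Flag tracks the closed state so neither move repeats; nothing in this graph calls the close event.
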(event `self.HoleInWall.OnComponentHit`
  (params (HitComponent :type "PrimitiveComponent Object Reference") (OtherActor :type "Actor Object Reference") (OtherComp :type "PrimitiveComponent Object Reference") (NormalImpulse :type "Vector Structure") (Hit :type "HitResult Structure (by ref)"))
  (if (`self.flag`)
    (if (== OtherActor (`GameplayStatics.GetPlayerPawn` 0))
      (`self.Open_Event`))))

(event `Open_Event`
  (if (`self.flag`)
    (`SceneComponent.K2_AddRelativeLocation` (`self.StaticMesh`) (0.0 0.0 150.0) false false)
    (set `self.flag` false)))

(event `Close_Event`
  (if (not (`self.flag`))
    (`SceneComponent.K2_AddRelativeLocation` (`self.StaticMesh`) (0.0 0.0 -150.0) false false)
    (set `self.flag` true)))

(fn `UserConstructionScript`)