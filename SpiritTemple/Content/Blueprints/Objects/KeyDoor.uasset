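; A door that unlocks and opens when a key actor hits it.
; On a hit from a BP_key while still closed, it destroys the key, triggers the open event, marks itself open and removes the Lock actor if valid.
; The open event eases the Door component to the Target's relative location and rotation over a short timed move.
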(event `self.ReceiveBeginPlay`)

(event `openDoor_Event`
  (bind (_target_location _target_rotation) (`KismetMathLibrary.BreakTransform` (`self.Target`)))
  (`KismetSystemLibrary.MoveComponentTo` (`self.door`) _target_location _target_rotation true true 1.0))

(event `self.door.OnComponentHit`
  (params (HitComponent :type "PrimitiveComponent Object Reference") (OtherActor :type "Actor Object Reference") (OtherComp :type "PrimitiveComponent Object Reference") (NormalImpulse :type "Vector Structure") (Hit :type "HitResult Structure (by ref)"))
  (bind _lock (`self.Lock`))
  (bind _asbp_key (cast `/Game/Blueprints/Interactables/Water/BP_key` OtherActor))
  (if (not (`self.isOpen`))
    (`self.K2_DestroyActor` _asbp_key)
    (`self.openDoor_Event`)
    (set `self.isOpen` true)
    (`/Engine/EditorBlueprintResources/StandardMacros.IsValid` _lock
      (:`Is Valid`
        (`self.K2_DestroyActor` _lock)))))

(fn `UserConstructionScript`)