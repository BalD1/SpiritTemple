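; SpeDoor is a door actor that slides its Door component between a closed position and two open positions.
; On BeginPlay it stores the door's relative transform as the closed position.
; Four events move it with eased one-second MoveComponentTo calls: open to Target, close back to the stored position, second open to TargetSecond, and second close back to Target.
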(event `self.ReceiveBeginPlay`
  (set `self.BasePos` (`SceneComponent.GetRelativeTransform` (`self.door`))))

(event `closeDoor_Event`
  (bind _basepos_location (`KismetMathLibrary.BreakTransform` (`self.BasePos`)))
  (`KismetSystemLibrary.MoveComponentTo` (`self.door`) _basepos_location (struct) true true 1.0))

(event `openDoor_Event`
  (bind _target_location (`KismetMathLibrary.BreakTransform` (`self.Target`)))
  (`KismetSystemLibrary.MoveComponentTo` (`self.door`) _target_location (struct) true true 1.0))

(event `openDoorSecond_Event`
  (bind _targetsecond_location (`KismetMathLibrary.BreakTransform` (`self.TargetSecond`)))
  (`KismetSystemLibrary.MoveComponentTo` (`self.door`) _targetsecond_location (struct) true true 1.0))

(event `closeDoorSecond_Event`
  (bind _target_location (`KismetMathLibrary.BreakTransform` (`self.Target`)))
  (`KismetSystemLibrary.MoveComponentTo` (`self.door`) _target_location (struct) true true 1.0))

(fn `UserConstructionScript`)