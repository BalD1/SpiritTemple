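; BP_TickingFlamable_Manager runs a timed puzzle over a group of TickingFlamable singles that opens a related door.
; The first DecrementCount starts a countdown that shrinks the plates' radius on Tick, resetting the flamables when time runs out.
; When the count reaches zero, it opens the door, animates the plate radius through a timeline, then destroys itself.
; AddSingle spawns new flamables, and StartCooldown schedules a delayed reset.
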(event `self.ReceiveTick`
  (params (DeltaSeconds :type "Float (single-precision)"))
  (if (`self.IsTicking`)
    (bind _output_get (set `self.Timer` (- (`self.Timer`) DeltaSeconds)))
    (if (<= _output_get 0.0)
      (`self.Reset`)
      (else
        (for _array_element (`self.Plates`)
          (`/Game/Blueprints/BP_TickingPlate.UpdateRadius` _array_element (/ (`/Game/Blueprints/BP_TickingPlate.M_RadiusMax` _array_element) (/ (`self.TimerMax`) (`self.Timer`)))))))))

(event `AddSingle`
  (bind _returnvalue (`|SpawnActorFromClass` "/Game/Blueprints/Interactables/Fire/BP_TickingFlamable_Single.BP_TickingFlamable_Single_C" (`self.GetTransform` self) "Undefined" "OverrideRootScale" null null))
  (`KismetArrayLibrary.Array_Add` (`self.TickingFlamables`) _returnvalue))

(event `DecrementCount`
  (bind _relateddoor (`self.RelatedDoor`))
  (if (not (`self.IsTicking`))
    (set `self.IsTicking` true)
    (set `self.Timer` (`self.TimerMax`)))
  (bind _result (`/Engine/EditorBlueprintResources/StandardMacros.DecrementInt` (`self.FlamablesCount`))
    (:`  `
      (if (<= _result 0)
        (set `self.End` true)
        (`/Engine/EditorBlueprintResources/StandardMacros.IsValid` _relateddoor
          (:`Is Valid`
            (`/Game/Blueprints/Interactables/BP_door.openDoor_Event` _relateddoor)
            (set `self.IsTicking` false)
            (bind (_direction _littrack) (`Timeline|LitPlates` :!via `PlayFromStart`)
              (:`Update`
                (for _array_element (`self.Plates`)
                  (`/Game/Blueprints/BP_TickingPlate.UpdateRadius` _array_element (+ (* (`/Game/Blueprints/BP_TickingPlate.M_RadiusMax` _array_element) _littrack) (`/Game/Blueprints/BP_TickingPlate.M_RadiusMin` _array_element)))))
              (:`Finished`
                (`self.K2_DestroyActor`)))))))))

(event `self.ReceiveBeginPlay`
  (`self.Reset`)
  (for _array_element (`self.TickingFlamables`)
    (set `/Game/Blueprints/Interactables/Fire/BP_TickingFlamable_Single.Manager` self _array_element)))

(event `StartCooldown`
  (`KismetSystemLibrary.K2_SetTimer` null "Reset" (`self.CoolDown`)))

(fn `Reset`
  (if (not (`self.End`))
    (for _array_element (`self.TickingFlamables`)
      (`/Game/Blueprints/Interactables/Fire/BP_TickingFlamable_Single.ChangeColor` _array_element false)
      (set `self.FlamablesCount` (`KismetArrayLibrary.Array_Length` (`self.TickingFlamables`)))
      (set `self.IsTicking` false))))

(fn `UserConstructionScript`)