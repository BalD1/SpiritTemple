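; Flammable wall actor that burns away when a fire projectile overlaps its cube mesh.
; The overlap plays a fire sound and effect, then after a short delay removes the cube, fades the sound and destroys the actor.
; While burning, Tick decays BurningValue exponentially per frame and feeds it to the cube materials' Burning scalar parameter, so the animation is frame-rate dependent.
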(event `self.Cube.OnComponentBeginOverlap`
  (params (OverlappedComponent :type "PrimitiveComponent Object Reference") (OtherActor :type "Actor Object Reference") (OtherComp :type "PrimitiveComponent Object Reference") (OtherBodyIndex :type Integer) (bFromSweep :type Boolean) (SweepResult :type "HitResult Structure (by ref)"))
  (cast `/Game/Blueprints/Powers/Projecties/BP_ProjectileFire` OtherActor)
  (bind _returnvalue (`GameplayStatics.SpawnSoundAtLocation` "/Game/StarterContent/Audio/Fire01.Fire01" (`SceneComponent.K2_GetComponentLocation` (`self.Fire`)) (struct) 0.8 1.0 0.0 null null))
  (set `self.FireSound` _returnvalue)
  (`ActorComponent.Activate` (`self.Fire`) false)
  (set `self.OnFire` true)
  (`KismetSystemLibrary.Delay` 1.5)
  (`ActorComponent.Deactivate` (`self.Fire`))
  (`ActorComponent.K2_DestroyComponent` (`self.Cube`))
  (set `self.OnFire` false)
  (`AudioComponent.FadeOut` (`self.FireSound`) 0.5 0.0 "Linear")
  (`KismetSystemLibrary.Delay` 2.0)
  (`self.K2_DestroyActor`))

(event `self.ReceiveTick`
  (params (DeltaSeconds :type "Float (single-precision)"))
  (if (`self.OnFire`)
    (set `self.Burning Value` (* (`self.Burning Value`) 0.99))
    (`MeshComponent.SetScalarParameterValueOnMaterials` (`self.Cube`) "Burning" (`self.Burning Value`))))

(fn `UserConstructionScript`)