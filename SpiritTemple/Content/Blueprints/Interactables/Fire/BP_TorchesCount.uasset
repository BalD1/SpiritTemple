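; BP_TorchesCount is a counter that opens a linked door when all of its related torches are lit.
; On BeginPlay it sets the unlit count from the RelatedTorches array length and sets each torch's RelatedCount to None.
; LitTorch lowers the count and opens RelatedDoor at zero.
; UnlitTorch closes the door if all torches were lit, then raises the count.
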(event `self.ReceiveBeginPlay`
  (bind _relatedtorches (`self.RelatedTorches`))
  (set `self.UnlitTorches` (`KismetArrayLibrary.Array_Length` _relatedtorches))
  (for _array_element _relatedtorches
    (set `/Game/Blueprints/Interactables/Fire/BP_Torch.RelatedCount` null _array_element)))

(event `LitTorch`
  (set `self.UnlitTorches` (- (`self.UnlitTorches`) 1))
  (if (== (`self.UnlitTorches`) 0)
    (`/Game/Blueprints/Interactables/BP_door.openDoor_Event` (`self.RelatedDoor`))))

(event `UnlitTorch`
  (if (== (`self.UnlitTorches`) 0)
    (`/Game/Blueprints/Interactables/BP_door.closeDoor_Event` (`self.RelatedDoor`)))
  (set `self.UnlitTorches` (+ (`self.UnlitTorches`) 1)))

(fn `UserConstructionScript`)