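; BP_Torch is an interactable torch that lights when a BP_ProjectileFire overlaps its trigger and can be put out through the UnlitTorch event.
; Each change of lit state toggles the fire particles and updates a linked RelatedCount counter, subtracting when lit and adding when unlit.
; Torches that start lit report to that counter after a short delay on BeginPlay, while unlit ones switch their particles off.
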(event `self.ReceiveBeginPlay`
  (if (`self.IsLit`)
    (`KismetSystemLibrary.Delay` 0.2)
    (`/Game/Blueprints/Interactables/BP_CounterBase.UpdateCounter` (`self.RelatedCount`) false self)
    (else
      (`ActorComponent.Deactivate` (`self.FireParticles`)))))

(event `self.Trigger.OnComponentBeginOverlap`
  (params (OverlappedComponent :type "PrimitiveComponent Object Reference") (OtherActor :type "Actor Object Reference") (OtherComp :type "PrimitiveComponent Object Reference") (OtherBodyIndex :type Integer) (bFromSweep :type Boolean) (SweepResult :type "HitResult Structure (by ref)"))
  (cast `/Game/Blueprints/Powers/Projecties/BP_ProjectileFire` OtherActor)
  (if (not (`self.IsLit`))
    (set `self.IsLit` true)
    (`/Game/Blueprints/Interactables/BP_CounterBase.UpdateCounter` (`self.RelatedCount`) false self)
    (`ActorComponent.Activate` (`self.FireParticles`) true)))

(event `UnlitTorch`
  (if (`self.IsLit`)
    (set `self.IsLit` false)
    (`/Game/Blueprints/Interactables/BP_CounterBase.UpdateCounter` (`self.RelatedCount`) true self)
    (`ActorComponent.Deactivate` (`self.FireParticles`))))

(fn `UserConstructionScript`)