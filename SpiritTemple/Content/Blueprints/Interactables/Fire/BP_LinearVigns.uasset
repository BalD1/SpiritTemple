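; Flammable vine segment that chains into straight lines and burns away when hit by a fire projectile.
; Editor events spawn linked segments at either end of the chain, roll the segment in quarter turns, and copy delay and burn settings to neighbors.
; Once lit, it waits an optional delay, ignites both neighbors so fire spreads along the chain, then drives the material's burn parameter by timeline and destroys itself.
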(event `AddVignFront`
  ;[1 1 1] Editor Events
  (`self.AddVign` true))

(event `AddVignBack`
  ;[1 1 1] Editor Events
  (`self.AddVign` false))

(event `Rotate`
  (bind _returnvalue_roll (`KismetMathLibrary.BreakRotator` (`SceneComponent.K2_GetComponentRotation` (`self.DefaultSceneRoot`))))
  ;[1 1 1] Editor Events
  (`SceneComponent.K2_SetRelativeRotation` (`self.DefaultSceneRoot`) (`KismetMathLibrary.MakeRotator` (+ _returnvalue_roll 90.0)) false false))

(event `LitVign`
  (bind _frontvign (`self.FrontVign`))
  (bind _backvign (`self.BackVign`))
  (if (not (`self.IsLit`))
    (bind _havedelay (`self.LitBehaviour` true))
    (if _havedelay
      (`KismetSystemLibrary.Delay` (`self.LitDelay`)))
    (`/Engine/EditorBlueprintResources/StandardMacros.IsValid` _frontvign
      (:`Is Valid`
        (`self.LitVign` _frontvign))
      (:`Is Not Valid`
        _))
    (`/Engine/EditorBlueprintResources/StandardMacros.IsValid` _backvign
      (:`Is Valid`
        (`self.LitVign` _backvign))
      (:`Is Not Valid`
        _))
    (`ActorComponent.Activate` (`self.Fire`) true)
    (bind (_direction _burn) (`Timeline|BurningRate` :!via `PlayFromStart`)
      (:`Update`
        (`MeshComponent.SetScalarParameterValueOnMaterials` (`self.Vign`) "Burning" _burn))
      (:`Finished`
        (`self.K2_DestroyActor`)))))

(event `self.ReceiveBeginPlay`
  (`ActorComponent.Deactivate` (`self.Fire`)))

(event `self.Vign.OnComponentBeginOverlap`
  (params (OverlappedComponent :type "PrimitiveComponent Object Reference") (OtherActor :type "Actor Object Reference") (OtherComp :type "PrimitiveComponent Object Reference") (OtherBodyIndex :type Integer) (bFromSweep :type Boolean) (SweepResult :type "HitResult Structure (by ref)"))
  (cast `/Game/Blueprints/Powers/Projecties/BP_ProjectileFire` OtherActor)
  (`self.LitVign`))

(event `Update Vars`
  (bind _frontvign (`self.FrontVign`))
  (bind _backvign (`self.BackVign`))
  (`/Engine/EditorBlueprintResources/StandardMacros.IsValid` _frontvign
    (:`Is Valid`
      (set `/Game/Blueprints/Interactables/Fire/BP_LinearVigns.LitDelay` (`self.LitDelay`) _frontvign)
      (set `/Game/Blueprints/Interactables/Fire/BP_LinearVigns.BurnTime` (`self.BurnTime`) _frontvign)
      (`self.Update Vars` _frontvign))
    (:`Is Not Valid`
      _))
  (`/Engine/EditorBlueprintResources/StandardMacros.IsValid` _backvign
    (:`Is Valid`
      (set `/Game/Blueprints/Interactables/Fire/BP_LinearVigns.LitDelay` (`self.LitDelay`) _backvign)
      (set `/Game/Blueprints/Interactables/Fire/BP_LinearVigns.BurnTime` (`self.BurnTime`) _backvign)
      (`self.Update Vars` _backvign))))

(fn `AddVign`
  (params (InFront :type Boolean))
  (bind _frontvign (`self.FrontVign`))
  (bind _backvign (`self.BackVign`))
  (if InFront
    ;[1 1 1] Check if there is not already a vign
    (`/Engine/EditorBlueprintResources/StandardMacros.IsValid` _frontvign
      (:`Is Valid`
        (`self.AddVign` _frontvign true))
      (:`Is Not Valid`
        (bind _returnvalue (`|SpawnActorFromClass` "BP_LinearVigns_C" (`KismetMathLibrary.MakeTransform` (+ (`self.K2_GetActorLocation`) (* (`self.GetActorRightVector` self) -100.0)) (`SceneComponent.RelativeRotation` (`self.DefaultSceneRoot`))) "Undefined" "OverrideRootScale" null null))
        (bind _output_get (set `self.FrontVign` _returnvalue))
        (set `/Game/Blueprints/Interactables/Fire/BP_LinearVigns.BackVign` self _output_get)
        (set `/Game/Blueprints/Interactables/Fire/BP_LinearVigns.LitDelay` (`self.LitDelay`) _output_get)
        (set `/Game/Blueprints/Interactables/Fire/BP_LinearVigns.BurnTime` (`self.BurnTime`) _output_get)))
    (else
      (`/Engine/EditorBlueprintResources/StandardMacros.IsValid` _backvign
        (:`Is Valid`
          (`self.AddVign` _backvign false))
        (:`Is Not Valid`
          (bind _returnvalue_2 (`|SpawnActorFromClass` "BP_LinearVigns_C" (`KismetMathLibrary.MakeTransform` (+ (`self.K2_GetActorLocation`) (* (`self.GetActorRightVector` self) 100.0)) (`SceneComponent.RelativeRotation` (`self.DefaultSceneRoot`))) "Undefined" "OverrideRootScale" null null))
          (bind _output_get_2 (set `self.BackVign` _returnvalue_2))
          (set `/Game/Blueprints/Interactables/Fire/BP_LinearVigns.FrontVign` self _output_get_2)
          (set `/Game/Blueprints/Interactables/Fire/BP_LinearVigns.LitDelay` (`self.LitDelay`) _output_get_2)
          (set `/Game/Blueprints/Interactables/Fire/BP_LinearVigns.BurnTime` (`self.BurnTime`) _output_get_2))))))

(fn `LitBehaviour`
  (params (LitState :type Boolean))
  (returns (HaveDelay :type Boolean))
  (set `self.IsLit` LitState)
  (if (> (`self.LitDelay`) 0.0)
    (return true)
    (else
      (return false))))

(fn `UserConstructionScript`)