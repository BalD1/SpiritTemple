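; BP_Crate_Small is a small crate among the Earth interactables, built on parent logic that it calls on BeginPlay and construction.
; On BeginPlay it casts the player pawn to FirstPersonCharacter and caches that character's PowerPoint.
; If the cast succeeds, it also records the Cube's world scale as BaseScale and the scene root's location as LastGoodPosition.
; Nothing in this file reads these cached values.
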(event `self.ReceiveBeginPlay`
  (`parent.ReceiveBeginPlay`)
  (bind _asfirst_person_character (cast `/Game/FirstPerson/Player/FirstPersonCharacter` (`GameplayStatics.GetPlayerPawn` 0)))
  (set `self.PlayerPowerPoint` (`/Game/FirstPerson/Player/FirstPersonCharacter.PowerPoint` _asfirst_person_character))
  (set `self.BaseScale` (`SceneComponent.K2_GetComponentScale` (`self.Cube`)))
  (set `self.LastGoodPosition` (`SceneComponent.K2_GetComponentLocation` (`self.DefaultSceneRoot`))))

(fn `UserConstructionScript`
  (`parent.UserConstructionScript`))