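; Interactable reset button that returns its linked crates to their starting or custom positions.
; A trigger shows the player an interact prompt while the button can be pushed.
; Interacting calls Reset on each related crate, passing per-crate custom positions when the array lengths match, otherwise a zero vector.
; The mesh moves to a target and back as press feedback, with pushing disabled until that finishes.
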(event `self.InteractEvent`
  (`self.UpdateInteractPrompt` false)
  (set `self.CanBePushed` false)
  (if (== (`KismetArrayLibrary.Array_Length` (`self.CustomPosition`)) (`KismetArrayLibrary.Array_Length` (`self.RelatedCrates`)))
    (for (_array_element _array_index) (`self.RelatedCrates`)
      (`/Game/Blueprints/Interactables/Earth/BP_Crate_Base.Reset` _array_element (`|GetArrayItem` (`self.CustomPosition`) _array_index))
      (`KismetSystemLibrary.MoveComponentTo` (`self.Mesh`) (`self.Target`) (struct) false false 0.5 :!label _label)
      (`KismetSystemLibrary.MoveComponentTo` (`self.Mesh`) (`self.BasePos`) (struct) false false 0.5)
      (set `self.CanBePushed` true))
    (else
      (for _array_element_2 (`self.RelatedCrates`)
        (`/Game/Blueprints/Interactables/Earth/BP_Crate_Base.Reset` _array_element_2 (0.0 0.0 0.0))
        (goto _label)))))

(event `self.ReceiveBeginPlay`
  (set `self.BasePos` (`SceneComponent.RelativeLocation` (`self.Mesh`))))

(event `self.Trigger.OnComponentBeginOverlap`
  (params (OverlappedComponent :type "PrimitiveComponent Object Reference") (OtherActor :type "Actor Object Reference") (OtherComp :type "PrimitiveComponent Object Reference") (OtherBodyIndex :type Integer) (bFromSweep :type Boolean) (SweepResult :type "HitResult Structure (by ref)"))
  (cast `/Game/FirstPerson/Player/FirstPersonCharacter` OtherActor)
  (if (`self.CanBePushed`)
    (`self.UpdateInteractPrompt` true "Press \"E\" to reset crates." (make `SlateColor` (struct :`R` 0.692708 :`G` 0.145292 :`B` 0.041453 :`A` 1.0)))))

(event `self.Trigger.OnComponentEndOverlap`
  (params (OverlappedComponent :type "PrimitiveComponent Object Reference") (OtherActor :type "Actor Object Reference") (OtherComp :type "PrimitiveComponent Object Reference") (OtherBodyIndex :type Integer))
  (cast `/Game/FirstPerson/Player/FirstPersonCharacter` OtherActor)
  (if (`self.CanBePushed`)
    (`self.UpdateInteractPrompt` false)))

(fn `UserConstructionScript`)