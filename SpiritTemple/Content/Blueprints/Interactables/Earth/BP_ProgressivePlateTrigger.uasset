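; BP_ProgressivePlateTrigger is a trigger actor that lights a referenced Plate when the first-person character or a BP_Crate_Base enters its volume.
; On overlap it validates the Plate, then either lights it instantly with Alpha or progressively adds Alpha over a set Time, depending on the InstantLit flag.
; The trigger can optionally destroy itself after its first successful use.
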(event `self.Trigger.OnComponentBeginOverlap`
  (params (OverlappedComponent :type "PrimitiveComponent Object Reference") (OtherActor :type "Actor Object Reference") (OtherComp :type "PrimitiveComponent Object Reference") (OtherBodyIndex :type Integer) (bFromSweep :type Boolean) (SweepResult :type "HitResult Structure (by ref)"))
  (bind _plate (`self.Plate`))
  (cast `/Game/FirstPerson/Player/FirstPersonCharacter` OtherActor
    (:`then`
      _)
    (:`CastFailed`
      (cast `/Game/Blueprints/Interactables/Earth/BP_Crate_Base` OtherActor)))
  (`/Engine/EditorBlueprintResources/StandardMacros.IsValid` _plate
    (:`Is Valid`
      (if (`self.InstantLit`)
        (`/Game/Blueprints/Plates/BP_ProgressivePlate.InstantLit` _plate (`self.Alpha`))
        (else
          (`/Game/Blueprints/Plates/BP_ProgressivePlate.ProgressiveLit` _plate (`self.Alpha`) (`self.Time`))))
      (if (`self.DestroyOnFirstUse`)
        (`self.K2_DestroyActor`)))))

(fn `UserConstructionScript`)