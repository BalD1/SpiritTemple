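; BP_button is an interactable push button that opens its linked door.
; A trigger volume shows or hides the interact prompt as the first-person character enters and leaves, while the button can still be pushed.
; InteractEvent calls the related door's open event, clears the prompt, disables further prompting and eases the button component to its target position.
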(event `self.trigger.OnComponentBeginOverlap`
  (params (OverlappedComponent :type "PrimitiveComponent Object Reference") (OtherActor :type "Actor Object Reference") (OtherComp :type "PrimitiveComponent Object Reference") (OtherBodyIndex :type Integer) (bFromSweep :type Boolean) (SweepResult :type "HitResult Structure (by ref)"))
  (cast `/Game/FirstPerson/Player/FirstPersonCharacter` OtherActor)
  (if (`self.CanBePushed`)
    (`self.UpdateInteractPrompt` true)))

(event `self.trigger.OnComponentEndOverlap`
  (params (OverlappedComponent :type "PrimitiveComponent Object Reference") (OtherActor :type "Actor Object Reference") (OtherComp :type "PrimitiveComponent Object Reference") (OtherBodyIndex :type Integer))
  (cast `/Game/FirstPerson/Player/FirstPersonCharacter` OtherActor)
  (if (`self.CanBePushed`)
    (`self.UpdateInteractPrompt` false)))

(event `self.InteractEvent`
  (`/Game/Blueprints/Interactables/BP_door.openDoor_Event` (`self.Related door`))
  (`self.UpdateInteractPrompt` false)
  (set `self.CanBePushed` false)
  (`KismetSystemLibrary.MoveComponentTo` (`self.button`) (`self.Target`) (struct) true true 1.0))

(fn `UserConstructionScript`)