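; One-shot lever interactable that opens a linked door or, if no valid door is set, a linked wall.
; Box overlap toggles the interact prompt for the player pawn.
; On interact, the mesh rotates through MoveComponentTo, OpenedFlag blocks reuse, and the target's open event fires.
; The door branch also lights an optional MagicalPath; with neither target valid, the lever does nothing.
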(event `self.Box.OnComponentBeginOverlap`
  (params (OverlappedComponent :type "PrimitiveComponent Object Reference") (OtherActor :type "Actor Object Reference") (OtherComp :type "PrimitiveComponent Object Reference") (OtherBodyIndex :type Integer) (bFromSweep :type Boolean) (SweepResult :type "HitResult Structure (by ref)"))
  (if (== OtherActor (`GameplayStatics.GetPlayerPawn` 0))
    (`self.UpdateInteractPrompt` true)))

(event `self.Box.OnComponentEndOverlap`
  (params (OverlappedComponent :type "PrimitiveComponent Object Reference") (OtherActor :type "Actor Object Reference") (OtherComp :type "PrimitiveComponent Object Reference") (OtherBodyIndex :type Integer))
  (if (== OtherActor (`GameplayStatics.GetPlayerPawn` 0))
    (`self.UpdateInteractPrompt` false)))

(event `self.InteractEvent`
  (bind _magical_path (`self.Magical Path`))
  (if (not (`self.Opened Flag`))
    (`/Engine/EditorBlueprintResources/StandardMacros.IsValid` (`self.Door`)
      (:`Is Valid`
        (`KismetSystemLibrary.MoveComponentTo` (`self.StaticMesh`) (0.0 0.0 0.0) (struct :`Pitch` -45.0))
        (set `self.Opened Flag` true)
        (`/Game/Blueprints/Objects/SpeDoor.openDoor_Event` (`self.Door`))
        (`/Engine/EditorBlueprintResources/StandardMacros.IsValid` _magical_path
          (:`Is Valid`
            (`/Game/Blueprints/BP_MagicalPath.LitPath` _magical_path))))
      (:`Is Not Valid`
        (`/Engine/EditorBlueprintResources/StandardMacros.IsValid` (`self.OpenWall`)
          (:`Is Valid`
            (`KismetSystemLibrary.MoveComponentTo` (`self.StaticMesh`) (0.0 0.0 0.0) (struct :`Pitch` -45.0))
            (set `self.Opened Flag` true)
            (`/Game/Blueprints/Objects/HoleInWall.Open_Event` (`self.OpenWall`))))))))

(fn `UserConstructionScript`
  (`parent.UserConstructionScript`))