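; A collectible gem that spins in place and, on its first Pickup, plays a sound, spins at its picked speed and scales by timeline until destroyed.
; Pickup also updates an optional related counter, while the timeline switches off the point light near zero scale and triggers an optional related plate after a delay.
; The construction script applies the gem color to mesh, light and the plate's lit color.
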(event `self.ReceiveTick`
  (params (DeltaSeconds :type "Float (single-precision)"))
  (bind (_returnvalue_roll _returnvalue_pitch _returnvalue_yaw) (`KismetMathLibrary.BreakRotator` (`SceneComponent.K2_GetComponentRotation` (`self.Mesh`))))
  (`parent.ReceiveTick` DeltaSeconds)
  (`SceneComponent.K2_SetWorldRotation` (`self.Mesh`) (`KismetMathLibrary.MakeRotator` _returnvalue_roll _returnvalue_pitch (+ _returnvalue_yaw (* DeltaSeconds (`self.RotationSpeed`)))) false false))

(event `self.Pickup`
  (bind _relatedplate (`self.RelatedPlate`))
  (if (not (`self.PickupFlag`))
    (bind _returnvalue (`GameplayStatics.SpawnSound2D` "/Game/Audio/Pickupgem.Pickupgem" 1.0 1.0 0.0 null))
    (set `self.SoundGem` _returnvalue)
    (set `self.PickupFlag` true)
    (set `self.RotationSpeed` (`self.PickedRotationSpeed`))
    (`/Engine/EditorBlueprintResources/StandardMacros.IsValid` (`self.RelatedCount`)
      (:`Is Valid`
        (`/Game/Blueprints/Interactables/BP_CounterBase.UpdateCounter` (`self.RelatedCount`) false self)
        (bind (_direction _scalevalue) (`Timeline|ScaleTimeline` :!via `PlayFromStart` :!label _label)
          (:`Update`
            (bind _returnvalue_2 (`KismetMathLibrary.Conv_DoubleToVector` _scalevalue))
            (`self.SetActorScale3D` _returnvalue_2)
            (if (== _returnvalue_2 (0.0 0.0 0.0) :`ErrorTolerance` 0.1)
              (`LightComponent.SetIntensity` (`self.PointLight`) 0.0))
            (`/Engine/EditorBlueprintResources/StandardMacros.IsValid` _relatedplate
              (:`Is Valid`
                (if (not (`self.PlateFlag`))
                  (`KismetSystemLibrary.Delay` (`self.PlateDelay`))
                  (`/Game/Blueprints/Plates/BP_PlateBase.UpdateState` _relatedplate)
                  (set `self.PlateFlag` true)))))
          (:`Finished`
            (`self.K2_DestroyActor`))))
      (:`Is Not Valid`
        (goto _label :!via `PlayFromStart`)))))

(fn `UserConstructionScript`
  (`parent.UserConstructionScript`)
  (`MeshComponent.SetVectorParameterValueOnMaterials` (`self.Mesh`) "Color" (`KismetMathLibrary.Conv_LinearColorToVector` (`self.GemColor`)))
  (`LightComponent.SetLightColor` (`self.PointLight`) (`self.GemColor`) true)
  (set `/Game/Blueprints/Plates/BP_PlateBase.LitColor` (`self.GemColor`) (`self.RelatedPlate`)))