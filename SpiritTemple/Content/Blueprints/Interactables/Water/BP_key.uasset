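; BP_key is a key interactable that the first-person player can pick up, carry and drop.
; Grab requires CanPlace and a camera-center trace hit, then a FlipFlop toggles between attaching the mesh to CratePoint and releasing it with physics.
; Trigger overlaps maintain an actor list that drives CanPlace.
; The material Color shows hover, carried and blocked states in green, white or red.
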(event `self.MouseHover`
  (if (not (`self.IsGrabbed`))
    (`MeshComponent.SetVectorParameterValueOnMaterials` (`self.Mesh`) "Color" (`KismetMathLibrary.Conv_LinearColorToVector` (`self.GreenColor`)))))

(event `self.MouseEndHover`
  (if (not (`self.IsGrabbed`))
    (`MeshComponent.SetVectorParameterValueOnMaterials` (`self.Mesh`) "Color" (1.0 1.0 1.0))))

(event `Grab`
  (bind _mesh (`self.Mesh`))
  ;[1 1 1] Cast a ray to check if Self is in view, and if Self can be placed
  (bind _asfirst_person_character (cast `/Game/FirstPerson/Player/FirstPersonCharacter` (`GameplayStatics.GetPlayerPawn` 0)))
  (bind _out_hit (`/Game/FirstPerson/Player/FirstPersonCharacter.TraceLineFromPlayerToCamCenter` _asfirst_person_character (struct :`R` 0.821501 :`B` 1.0 :`A` 1.0) 20000.0))
  (if (and (`self.CanPlace`) (== (`.HitActor` (`GameplayStatics.BreakHitResult` _out_hit)) self))
    (bind _isa (`/Engine/EditorBlueprintResources/StandardMacros.FlipFlop`)
      (:`A`
        ;[1 1 1] Attach to the player
        (set `self.IsGrabbed` _isa)
        (bind _asfirst_person_character_2 (cast `/Game/FirstPerson/Player/FirstPersonCharacter` (`GameplayStatics.GetPlayerPawn` 0)))
        (`PrimitiveComponent.SetSimulatePhysics` (`self.Mesh`) false)
        (`SceneComponent.K2_AttachToComponent` _mesh (`/Game/FirstPerson/Player/FirstPersonCharacter.CratePoint` _asfirst_person_character_2) "None" "SnapToTarget" "SnapToTarget" "KeepWorld" true)
        (`self.SetCanPlace` true))
      (:`B`
        ;[1 1 1] Detach from player
        (set `self.IsGrabbed` _isa)
        (`SceneComponent.K2_DetachFromComponent` _mesh "KeepWorld" "KeepWorld" "KeepWorld" true)
        (`PrimitiveComponent.SetSimulatePhysics` (`self.Mesh`) true)
        (`self.SetCanPlace` (`self.CanPlace`))))))

(event `self.Trigger.OnComponentBeginOverlap`
  (params (OverlappedComponent :type "PrimitiveComponent Object Reference") (OtherActor :type "Actor Object Reference") (OtherComp :type "PrimitiveComponent Object Reference") (OtherBodyIndex :type Integer) (bFromSweep :type Boolean) (SweepResult :type "HitResult Structure (by ref)"))
  ;[1 1 1] If touches another actor, Self can't be placed
  (`KismetArrayLibrary.Array_Add` (`self.OverlappingActors`) OtherActor)
  (`self.SetCanPlace` false))

(event `self.Trigger.OnComponentEndOverlap`
  (params (OverlappedComponent :type "PrimitiveComponent Object Reference") (OtherActor :type "Actor Object Reference") (OtherComp :type "PrimitiveComponent Object Reference") (OtherBodyIndex :type Integer))
  (bind _overlappingactors (`self.OverlappingActors`))
  ;[1 1 1] If doesn't touches ANY other actor, Self can be placed
  (`KismetArrayLibrary.Array_RemoveItem` _overlappingactors OtherActor)
  (if (<= (`KismetArrayLibrary.Array_Length` _overlappingactors) 0)
    (`self.SetCanPlace` true)))

(fn `SetCanPlace`
  (params (NewCanPlace :type Boolean))
  (bind _output_get (set `self.CanPlace` NewCanPlace))
  (if _output_get
    (if (`self.IsGrabbed`)
      (`MeshComponent.SetVectorParameterValueOnMaterials` (`self.Mesh`) "Color" (`KismetMathLibrary.Conv_LinearColorToVector` (`self.GreenColor`)))
      (else
        (`MeshComponent.SetVectorParameterValueOnMaterials` (`self.Mesh`) "Color" (1.0 1.0 1.0))))
    (else
      (`MeshComponent.SetVectorParameterValueOnMaterials` (`self.Mesh`) "Color" (`KismetMathLibrary.Conv_LinearColorToVector` (`self.RedColor`))))))

(fn `UserConstructionScript`)