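; BP_KeyItemCounter opens a linked door once every key item assigned to it has been picked up.
; On BeginPlay it counts the RelatedItems array and registers itself as each item's RelatedCount.
; ItemPickedUp decrements the count and calls OpenDoorEvent on RelatedDoor when it reaches zero.
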(event `self.ReceiveBeginPlay`
  (bind _relateditems (`self.RelatedItems`))
  (set `self.ItemsCount` (`KismetArrayLibrary.Array_Length` _relateditems))
  (for _array_element _relateditems
    (set `/Game/Blueprints/Interactables/Water/BP_PickableObjectBase.RelatedCount` self _array_element)))

(event `ItemPickedUp`
  (bind _result (`/Engine/EditorBlueprintResources/StandardMacros.DecrementInt` (`self.ItemsCount`))
    (:`  `
      (if (== _result 0)
        (`/Game/Blueprints/Interactables/BP_door.openDoor_Event` (`self.RelatedDoor`))))))

(fn `UserConstructionScript`)