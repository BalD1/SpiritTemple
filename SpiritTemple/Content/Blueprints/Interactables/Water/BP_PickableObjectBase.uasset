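; BP_PickableObjectBase is a base pickup that can home in on the player and collect itself on contact.
; Once StartMoving is called, each Tick moves it straight toward the player character at Speed, scaled by delta time, without sweeping.
; When FirstPersonCharacter overlaps the Trigger, Pickup notifies RelatedCount that an item was picked up, then destroys the actor.
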(event `self.Trigger.OnComponentBeginOverlap`
  (params (OverlappedComponent :type "PrimitiveComponent Object Reference") (OtherActor :type "Actor Object Reference") (OtherComp :type "PrimitiveComponent Object Reference") (OtherBodyIndex :type Integer) (bFromSweep :type Boolean) (SweepResult :type "HitResult Structure (by ref)"))
  (cast `/Game/FirstPerson/Player/FirstPersonCharacter` OtherActor)
  (`self.Pickup`))

(event `Pickup`
  (`/Game/Blueprints/Interactables/Water/BP_KeyItemCounter.ItemPickedUp` (`self.RelatedCount`))
  (`self.K2_DestroyActor`))

(event `StartMoving`
  (set `self.CanMove` true))

(event `self.ReceiveTick`
  (params (DeltaSeconds :type "Float (single-precision)"))
  (if (`self.CanMove`)
    (`self.GoToPlayer`)))

(fn `GoToPlayer`
  (bind _returnvalue (`self.K2_GetActorLocation`))
  (`self.K2_SetActorLocation` (+ _returnvalue (* (* (`KismetMathLibrary.Normal` (- (`self.K2_GetActorLocation` (`GameplayStatics.GetPlayerCharacter` 0)) _returnvalue)) (`GameplayStatics.GetWorldDeltaSeconds`)) (`self.Speed`)))))

(fn `UserConstructionScript`)