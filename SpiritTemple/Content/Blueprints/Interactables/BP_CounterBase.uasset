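; BP_CounterBase is an interactable counter that sits between a group of activators and a door, aggregating their states.
; On BeginPlay it registers itself with each related torch or pickable object and counts them.
; UpdateCounter raises or lowers the count, telling RelatedDoor to add the counter as an activator when the count drops below one.
; An increment landing at one or below sends the door the opposite update.
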(event `self.ReceiveBeginPlay`
  (for _array_element (`self.RelatedActivators`)
    (bind _asbp_torch (cast `/Game/Blueprints/Interactables/Fire/BP_Torch` _array_element)
      (:`then`
        (set `/Game/Blueprints/Interactables/Fire/BP_Torch.RelatedCount` self _asbp_torch)
        (`/Engine/EditorBlueprintResources/StandardMacros.IncrementInt` (`self.Count`)))
      (:`CastFailed`
        (bind _asbp_pickable_object_base (cast `/Game/Blueprints/Interactables/Water/BP_PickableObjectBase` _array_element))
        (set `/Game/Blueprints/Interactables/Water/BP_PickableObjectBase.RelatedCount` self _asbp_pickable_object_base)
        (`/Engine/EditorBlueprintResources/StandardMacros.IncrementInt` (`self.Count`))))))

(fn `UpdateCounter`
  (params (Add :type Boolean) (Activator :type "Actor Object Reference"))
  (bind _count (`self.Count`))
  (if Add
    (bind _result (`/Engine/EditorBlueprintResources/StandardMacros.IncrementInt` _count)
      (:`  `
        (if (<= _result 1)
          (`/Game/Blueprints/Interactables/BP_door.ActivatorUpdate` (`self.RelatedDoor`) false self))))
    (else
      (bind _result_2 (`/Engine/EditorBlueprintResources/StandardMacros.DecrementInt` _count)
        (:`  `
          (if (< _result_2 1)
            (`/Game/Blueprints/Interactables/BP_door.ActivatorUpdate` (`self.RelatedDoor`) true self)))))))

(fn `UserConstructionScript`)