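; Interactable sliding door that opens while at least one activator is registered and closes when the last one leaves.
; ActivatorUpdate tracks the activator list and fires the open or close event on first add and last removal.
; Opening can trigger an optional cutscene once, wait out its blend time, then ease the door to its target location.
; Closing eases it back to the position saved at BeginPlay and resets the cutscene flag.
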(event `self.ReceiveBeginPlay`
  (set `self.BasePos` (`SceneComponent.GetRelativeTransform` (`self.door`))))

(event `closeDoor_Event`
  (bind _basepos_location (`KismetMathLibrary.BreakTransform` (`self.BasePos`)))
  (`KismetSystemLibrary.MoveComponentTo` (`self.door`) _basepos_location (struct) true true 1.0)
  (set `self.CutsceneFlag` false))

(event `openDoor_Event`
  (bind _target_location (`KismetMathLibrary.BreakTransform` (`self.Target`)))
  (bind _cutscene (`self.Cutscene`))
  (if (and (and (`KismetSystemLibrary.IsValid` (`self.Cutscene`)) (`self.CanCallCutscene`)) (not (`self.CutsceneFlag`)))
    (`/Game/Blueprints/BP_PuzzleResolve.CallCutscene` _cutscene)
    (set `self.CutsceneFlag` true)
    (`KismetSystemLibrary.Delay` (`/Game/Blueprints/BP_PuzzleResolve.Blend Time` _cutscene)))
  (`KismetSystemLibrary.MoveComponentTo` (`self.door`) _target_location (struct) true true 1.0))

(fn `ActivatorUpdate`
  (params (Add :type Boolean) (Actor :type "Actor Object Reference"))
  (bind _currentactivators (`self.CurrentActivators`))
  (if Add
    (bind _returnvalue (`KismetArrayLibrary.Array_Add` (`self.CurrentActivators`) Actor))
    ;[1 1 1] If the new activator is the only current one
    (if (== _returnvalue 0)
      (`self.openDoor_Event`))
    (else
      (`KismetArrayLibrary.Array_RemoveItem` _currentactivators Actor)
      ;[1 1 1] If the array is empty
      (if (< (`KismetArrayLibrary.Array_Length` _currentactivators) 1)
        (`self.closeDoor_Event`)))))

(fn `UserConstructionScript`)