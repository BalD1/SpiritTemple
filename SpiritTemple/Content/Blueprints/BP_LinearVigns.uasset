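; BP_LinearVigns is a vine-like "Vign" segment that lights up when the first-person character overlaps its box.
; Lighting swaps in the lit material, then spreads through the Front and Back links after an optional delay, with an IsLit guard stopping repeats.
; Editor events build the chain by spawning linked neighbours at fixed Y offsets in empty slots, and a Rotate event adjusts the mesh yaw.
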(event `AddVignFront`
  ;[1 1 1] Editor Events
  (`self.AddVign` true))

(event `AddVignBack`
  ;[1 1 1] Editor Events
  (`self.AddVign` false))

(event `Rotate`
  (bind (_returnvalue_roll _returnvalue_pitch _returnvalue_yaw) (`KismetMathLibrary.BreakRotator` (`SceneComponent.K2_GetComponentRotation` (`self.Vign`))))
  ;[1 1 1] Editor Events
  (`/Engine/EditorBlueprintResources/StandardMacros.IsValid` null
    (:`Is Not Valid`
      (`SceneComponent.K2_SetRelativeRotation` (`self.Vign`) (`KismetMathLibrary.MakeRotator` 0.0 0.0 (+ _returnvalue_yaw 90.0)) false false))))

(event `LitVign`
  (bind (_front _back) (break `/Game/Blueprints/STRUCT_LinearVigns` (`self.Related Vigns`)))
  (if (not (`self.IsLit`))
    (bind _havedelay (`self.LitBehaviour` true))
    (if _havedelay
      (`KismetSystemLibrary.Delay` (`self.LitDelay`)))
    (`/Engine/EditorBlueprintResources/StandardMacros.IsValid` _front
      (:`Is Valid`
        (`self.LitVign` _front))
      (:`Is Not Valid`
        _))
    (`/Engine/EditorBlueprintResources/StandardMacros.IsValid` _back
      (:`Is Valid`
        (`self.LitVign` _back)))))

(event `self.Box.OnComponentBeginOverlap`
  (params (OverlappedComponent :type "PrimitiveComponent Object Reference") (OtherActor :type "Actor Object Reference") (OtherComp :type "PrimitiveComponent Object Reference") (OtherBodyIndex :type Integer) (bFromSweep :type Boolean) (SweepResult :type "HitResult Structure (by ref)"))
  (cast `/Game/FirstPerson/Player/FirstPersonCharacter` OtherActor)
  (`self.LitVign`))

(fn `AddVign`
  (params (InFront :type Boolean))
  (bind (_front _back) (break `/Game/Blueprints/STRUCT_LinearVigns` (`self.RelatedVigns`)))
  (if InFront
    ;[1 1 1] Check if there is not already a vign
    (`/Engine/EditorBlueprintResources/StandardMacros.IsValid` _front
      (:`Is Not Valid`
        (bind _returnvalue (`|SpawnActorFromClass` "BP_LinearVigns_C" (`KismetMathLibrary.MakeTransform` (+ (`self.K2_GetActorLocation`) (0.0 -100.0 0.0))) "Undefined" "OverrideRootScale" null null))
        (setmembers `/Game/Blueprints/STRUCT_LinearVigns` :`StructRef` (`self.RelatedVigns`) :`Front` _returnvalue)
        (setmembers `/Game/Blueprints/STRUCT_LinearVigns` :`StructRef` (`/Game/Blueprints/BP_LinearVigns.RelatedVigns` _returnvalue) :`Back` self)))
    (else
      (`/Engine/EditorBlueprintResources/StandardMacros.IsValid` _back
        (:`Is Not Valid`
          (bind _returnvalue_2 (`|SpawnActorFromClass` "BP_LinearVigns_C" (`KismetMathLibrary.MakeTransform` (+ (`self.K2_GetActorLocation`) (0.0 100.0 0.0))) "Undefined" "OverrideRootScale" null null))
          (setmembers `/Game/Blueprints/STRUCT_LinearVigns` :`StructRef` (`self.RelatedVigns`) :`Back` _returnvalue_2)
          (setmembers `/Game/Blueprints/STRUCT_LinearVigns` :`StructRef` (`/Game/Blueprints/BP_LinearVigns.RelatedVigns` _returnvalue_2) :`Front` self))))))

(fn `Change Material`
  (`PrimitiveComponent.SetMaterial` (`self.Vign`) 0 (`self.LitMaterial`)))

(fn `LitBehaviour`
  (params (LitState :type Boolean))
  (returns (HaveDelay :type Boolean))
  (set `self.IsLit` LitState)
  (`self.Change Material`)
  (if (> (`self.LitDelay`) 0.0)
    (return true)
    (else
      (return false))))

(fn `UserConstructionScript`)