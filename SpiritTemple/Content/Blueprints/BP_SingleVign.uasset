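; BP_SingleVign is a single cell of a grid that toggles between lit and unlit states.
; Lit swaps the Cube's material to ComputeNormal and reports the cell's PositionInGrid to its Grid through LitVign.
; Unlit restores the base material without notifying the Grid, and an IsLit flag keeps both events from repeating on a cell already in that state.
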(event `Lit`
  (if (not (`self.IsLit`))
    (`PrimitiveComponent.SetMaterial` (`self.Cube`) 0 "/Game/Blueprints/BlueprintFluidSurface/ComputeNormal.ComputeNormal")
    (`/Game/Blueprints/BP_VignGrid.LitVign` (`self.Grid`) (`self.PositionInGrid`))
    (set `self.IsLit` true)))

(event `Unlit`
  (if (`self.IsLit`)
    (`PrimitiveComponent.SetMaterial` (`self.Cube`) 0 "/Game/FirstPerson/Meshes/BaseMaterial.BaseMaterial")
    (set `self.IsLit` false)))

(fn `UserConstructionScript`)