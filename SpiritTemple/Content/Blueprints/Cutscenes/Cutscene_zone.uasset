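; Trigger zone actor that plays a timed camera cutscene when the player character enters its box.
; On overlap it blends the view to SceneCamera and arms a countdown from CutsceneTime.
; While the countdown runs, Tick disables input and hides the pawn, then blends back and unhides it after a Delay.
; Whenever the cutscene flag is off, Tick re-enables player input every frame.
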(event `self.Box.OnComponentBeginOverlap`
  (params (OverlappedComponent :type "PrimitiveComponent Object Reference") (OtherActor :type "Actor Object Reference") (OtherComp :type "PrimitiveComponent Object Reference") (OtherBodyIndex :type Integer) (bFromSweep :type Boolean) (SweepResult :type "HitResult Structure (by ref)"))
  (if (== OtherActor (`GameplayStatics.GetPlayerCharacter` 0))
    (set `self.CamTimer` (`self.CutsceneTime`))
    (set `self.CamFlag` true)
    (`PlayerController.SetViewTargetWithBlend` (`GameplayStatics.GetPlayerController` 0) (`self.SceneCamera`) (`self.BlendTime`) "VTBlend_Linear" 0.0 true)))

(event `self.ReceiveTick`
  (params (DeltaSeconds :type "Float (single-precision)"))
  (bind _returnvalue (`GameplayStatics.GetPlayerController` 0))
  (bind _returnvalue_2 (`GameplayStatics.GetPlayerPawn` 0))
  (bind _returnvalue_3 (- (`self.CamTimer`) DeltaSeconds))
  (if (`self.CamFlag`)
    (`self.DisableInput` _returnvalue_2 _returnvalue)
    (`self.SetActorHiddenInGame` (`GameplayStatics.GetPlayerPawn` 0) true)
    (if (< _returnvalue_3 0.0)
      (`PlayerController.SetViewTargetWithBlend` (`GameplayStatics.GetPlayerController` 0) (`GameplayStatics.GetPlayerPawn` 0) (`self.BlendTime`) "VTBlend_Linear" 0.0 false)
      (`KismetSystemLibrary.Delay` (`self.BlendTime`))
      (set `self.CamFlag` false)
      (`self.SetActorHiddenInGame` (`GameplayStatics.GetPlayerPawn` 0) false)
      (else
        (set `self.CamTimer` _returnvalue_3)))
    (else
      (`self.EnableInput` _returnvalue_2 _returnvalue))))

(fn `UserConstructionScript`)