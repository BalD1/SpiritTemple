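; BP_MagicalStep_Var is a magical step variant that, when the first-person character overlaps its trigger, moves the next step in its chain into place.
; The linked RelatedStep's mesh eases to its Target over half a second if that step is movable.
; AddSingleStep recurses down the RelatedStep links to spawn and link a new step at the tail, and AddMultipleSteps repeats it.
; Construction disables two inherited flags before running the parent's script.
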(event `self.Trigger.OnComponentBeginOverlap`
  (params (OverlappedComponent :type "PrimitiveComponent Object Reference") (OtherActor :type "Actor Object Reference") (OtherComp :type "PrimitiveComponent Object Reference") (OtherBodyIndex :type Integer) (bFromSweep :type Boolean) (SweepResult :type "HitResult Structure (by ref)"))
  (bind _relatedstep (`self.RelatedStep`))
  (cast `/Game/FirstPerson/Player/FirstPersonCharacter` OtherActor)
  (`/Engine/EditorBlueprintResources/StandardMacros.IsValid` _relatedstep
    (:`Is Valid`
      (bind _asbp_magical_step_var (cast `/Game/Blueprints/BP_MagicalStep_Var` _relatedstep))
      (if (`/Game/Blueprints/BP_MagicalStep_Var.IsMovable` _asbp_magical_step_var)
        (`KismetSystemLibrary.MoveComponentTo` (`/Game/Blueprints/BP_MagicalStep.StaticMesh` _asbp_magical_step_var) (`/Game/Blueprints/BP_MagicalStep_Var.Target` _asbp_magical_step_var) (struct) true true 0.5)))))

(event `self.Add multiple steps`
  (for _ (range (`self.Steps to add`))
    (`self.Add single step`)))

(event `self.Add single step`
  (`/Engine/EditorBlueprintResources/StandardMacros.IsValid` (`self.RelatedStep`)
    (:`Is Valid`
      (`self.Add single step` (`self.RelatedStep`)))
    (:`Is Not Valid`
      (bind _returnvalue (`|SpawnActorFromClass` "BP_MagicalStep_Var_C" (`self.GetTransform`) "Undefined" "OverrideRootScale" null null))
      (set `self.RelatedStep` _returnvalue)
      (`self.Update Related Steps`))))

(fn `UserConstructionScript`
  (set `self.M_RadiusAtMin` false)
  (set `self.MustDisappearOnEndOverlapp` false)
  (`parent.UserConstructionScript`))