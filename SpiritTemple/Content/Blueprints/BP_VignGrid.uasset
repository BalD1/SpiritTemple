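; Grid actor that spawns and tracks BP_SingleVign actors at listed cells of a 2D integer grid.
; SpawnVigns clears the previous set, then places each vign at cell times VignSize from the actor's location, passing it its cell and grid reference.
; UpdateGrid adds a coordinate text label for every cell.
; Small int-vector helpers handle the math; LitVign and CheckNeighbors are unfinished stubs for neighbor checks.
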(event `Spawn Vigns`
  (bind _gridsize_x (break `/Game/Blueprints/IntVector2` (`self.GridSize`)))
  (bind (_gridsize_x_2 _gridsize_y) (break `/Game/Blueprints/IntVector2` (`self.GridSize`)))
  (`self.ClearVigns`)
  (for _index (range (+ _gridsize_x 1))
    (for _index_2 (range (+ _gridsize_y 1))
      (for _array_element _
        (bind _intvector2 (make `/Game/Blueprints/IntVector2` _index _index_2))
        (bind (_isequal _vector) (`self.IntVectorEquals` _intvector2 _array_element))
        (if _isequal
          (bind _result (`self.Multiply Int Vector2` _vector (`self.VignSize`)))
          (bind _returnvalue (`|SpawnActorFromClass` "/Game/Blueprints/BP_SingleVign.BP_SingleVign_C" (`KismetMathLibrary.MakeTransform` (+ (`KismetMathLibrary.MakeVector` (`KismetMathLibrary.Conv_IntToDouble` (break `/Game/Blueprints/IntVector2` _result)) (`KismetMathLibrary.Conv_IntToDouble` (`.Y_4_86BA68DE4F38406342937E91C394348F` (break `/Game/Blueprints/IntVector2` _result)))) (`self.K2_GetActorLocation`))) "Undefined" "OverrideRootScale" null null))
          (`KismetArrayLibrary.Array_Add` (`self.VignsTable`) _returnvalue)
          (set `/Game/Blueprints/BP_SingleVign.PositionInGrid` _intvector2 _returnvalue)
          (set `/Game/Blueprints/BP_SingleVign.Grid` self _returnvalue))))))

(event `ClearVigns`
  (bind _vignstable (`self.VignsTable`))
  (for _array_element _vignstable
    (`self.K2_DestroyActor` _array_element))
  (`KismetArrayLibrary.Array_Clear` _vignstable))

(event `Update Grid`
  (bind _gridsize_x (break `/Game/Blueprints/IntVector2` (`self.GridSize`)))
  (bind (_gridsize_x_2 _gridsize_y) (break `/Game/Blueprints/IntVector2` (`self.GridSize`)))
  (for _index (range (+ _gridsize_x 1))
    (for _index_2 (range (+ _gridsize_y 1))
      (bind _intvector2 (make `/Game/Blueprints/IntVector2` _index _index_2))
      (bind _result (`self.Multiply Int Vector2` _intvector2 (`self.VignSize`)))
      (bind _returnvalue (`AddComponent|NODE_AddTextRenderComponent-0` :`RelativeTransform` (`KismetMathLibrary.MakeTransform` (`KismetMathLibrary.MakeVector` (`KismetMathLibrary.Conv_IntToDouble` (break `/Game/Blueprints/IntVector2` _result)) (`KismetMathLibrary.Conv_IntToDouble` (`.Y_4_86BA68DE4F38406342937E91C394348F` (break `/Game/Blueprints/IntVector2` _result)))))))
      (bind (_x _y) (break `/Game/Blueprints/IntVector2` _intvector2))
      (`TextRenderComponent.K2_SetText` _returnvalue (`KismetTextLibrary.Conv_StringToText` (`KismetStringLibrary.Concat_StrStr` (`KismetStringLibrary.Conv_IntToString` _x) "," (`KismetStringLibrary.Conv_IntToString` _y))))
      (`TextRenderComponent.SetHorizontalAlignment` _returnvalue "EHTA_Center"))))

(event `LitVign`
  (params (VignPosition :type "/Game/Blueprints/IntVector2 Structure"))
  (for _array_element _
    (`self.Add Int Vector2` VignPosition (make `/Game/Blueprints/IntVector2` 1))
    (`self.IntVectorEquals` _array_element)
    (if true
      _)))

(fn `Add Int Vector2`
  (params (A :type "/Game/Blueprints/IntVector2 Structure") (B :type "/Game/Blueprints/IntVector2 Structure"))
  (returns (Output :type "/Game/Blueprints/IntVector2 Structure"))
  (return (make `/Game/Blueprints/IntVector2` (+ A_X_2_8BC538FD449BC2A550533498F5EDB174 B_X_2_8BC538FD449BC2A550533498F5EDB174) (+ A_Y_4_86BA68DE4F38406342937E91C394348F B_Y_4_86BA68DE4F38406342937E91C394348F))))

(fn `CheckNeighbors`
  (params (StartPosition :type "/Game/Blueprints/IntVector2 Structure")))

(fn `IntVectorEquals`
  (params (A :type "/Game/Blueprints/IntVector2 Structure") (B :type "/Game/Blueprints/IntVector2 Structure"))
  (returns (IsEqual :type Boolean) (Vector :type "/Game/Blueprints/IntVector2 Structure"))
  (return (and (== A_X_2_8BC538FD449BC2A550533498F5EDB174 B_X_2_8BC538FD449BC2A550533498F5EDB174) (== A_Y_4_86BA68DE4F38406342937E91C394348F B_Y_4_86BA68DE4F38406342937E91C394348F)) (make `/Game/Blueprints/IntVector2` A_X_2_8BC538FD449BC2A550533498F5EDB174 A_Y_4_86BA68DE4F38406342937E91C394348F)))

(fn `Multiply Int Vector2`
  (params (A :type "/Game/Blueprints/IntVector2 Structure") (B :type "/Game/Blueprints/IntVector2 Structure"))
  (returns (Result :type "/Game/Blueprints/IntVector2 Structure"))
  (return (make `/Game/Blueprints/IntVector2` (* A_X_2_8BC538FD449BC2A550533498F5EDB174 B_X_2_8BC538FD449BC2A550533498F5EDB174) (* A_Y_4_86BA68DE4F38406342937E91C394348F B_Y_4_86BA68DE4F38406342937E91C394348F))))

(fn `UserConstructionScript`)