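; BP_ChakraBall_Stand is a stand that spawns a chakra ball for one of the seven chakras at its BallPoint, optionally on BeginPlay.
; SpawnChakra replaces any existing ball, picks a material by chakra type, and passes the name, item state, related plate and holder to the new BP_ChakraBall_Base.
; AnimateChakra runs the ball's sequence animation while a timeline drives the point light, then destroys the light; SkipCutscene picks up the ball and removes the light immediately.
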(event `self.ReceiveBeginPlay`
  (`/Engine/EditorBlueprintResources/StandardMacros.IsValid` (`self.SpawnedChakra`)
    (:`Is Not Valid`
      (if (`self.Spawn on start`)
        (`self.SpawnChakra`)))))

(event `SpawnChakra`
  (bind _spawnedchakra (`self.SpawnedChakra`))
  ;[1 1 1] Yes it is dégueulasse but c'est not grave, ça nous allow d'être lazy
  (`/Engine/EditorBlueprintResources/StandardMacros.IsValid` _spawnedchakra
    (:`Is Valid`
      (`self.K2_DestroyActor` _spawnedchakra))
    (:`Is Not Valid`
      _))
  (switch `/Game/Blueprints/Chakras/ENUM_ChakrasNames` (`self.Chakra`)
    (:`NewEnumerator0`
      (set `self.Material` "/Game/Materials/Chakras/M_Chakra_Muladhara.M_Chakra_Muladhara"))
    (:`NewEnumerator1`
      (set `self.Material` "/Game/Materials/Chakras/M_Chakra_Swadhistana.M_Chakra_Swadhistana"))
    (:`NewEnumerator2`
      (set `self.Material` "/Game/Materials/Chakras/M_Chakra_Manipura.M_Chakra_Manipura"))
    (:`NewEnumerator3`
      (set `self.Material` "/Game/Materials/Chakras/M_Chakra_Anahata.M_Chakra_Anahata"))
    (:`NewEnumerator4`
      (set `self.Material` "/Game/Materials/Chakras/M_ChakraVishuda.M_ChakraVishuda"))
    (:`NewEnumerator5`
      (set `self.Material` "/Game/Materials/Chakras/M_ChakraAjna.M_ChakraAjna"))
    (:`NewEnumerator6`
      (set `self.Material` "/Game/Materials/Chakras/M_Chakra_Sahasrara.M_Chakra_Sahasrara")))
  (bind _returnvalue (`|SpawnActorFromClass` "/Game/Blueprints/Chakras/BP_ChakraBall_Base.BP_ChakraBall_Base_C" (`SceneComponent.K2_GetComponentToWorld` (`self.BallPoint`)) "Undefined" "OverrideRootScale" null null))
  (set `self.SpawnedChakra` _returnvalue)
  (set `/Game/Blueprints/Chakras/BP_ChakraBall_Base.Name` (`self.Chakra`) _returnvalue)
  (`/Game/Blueprints/Chakras/BP_ChakraBall_Base.ResetMaterial` _returnvalue (`self.Material`))
  (`/Game/Blueprints/Chakras/BP_ChakraBall_Base.ResetIsItem` _returnvalue true)
  (set `/Game/Blueprints/Chakras/BP_ChakraBall_Base.RelatedPlate` (`self.RelatedPlate`) _returnvalue)
  (set `/Game/Blueprints/Chakras/BP_ChakraBall_Base.RelatedHolder` (`self.RelatedHolder`) _returnvalue))

(event `AnimateChakra`
  (`/Game/Blueprints/Chakras/BP_ChakraBall_Base.SequenceAnimation` (`self.SpawnedChakra`))
  (bind (_direction _intensity) (`Timeline|LightIntensity` :!via `PlayFromStart`)
    (:`Update`
      (`LightComponent.SetIntensity` (`self.PointLight`) _intensity))
    (:`Finished`
      (`ActorComponent.K2_DestroyComponent` (`self.PointLight`) :!label _label))))

(event `SkipCutscene`
  (`/Game/Blueprints/Chakras/BP_ChakraBall_Base.Pickup` (`self.SpawnedChakra`))
  (goto _label))

(fn `UserConstructionScript`)