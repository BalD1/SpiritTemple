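; Base chakra holder: an interactable socket where the player places a chakra from their inventory.
; A translucent-or-tinted ghost ball previews placement, changing color and toggling the interact prompt on cursor hover or interactability changes.
; Interacting swaps the ghost for a real ball, disables sphere collision and removes the chakra from the inventory.
; It then spawns a power on the linked PowerStand or, without one, ends the game if flagged.
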(event `self.ReceiveBeginPlay`
  (`parent.ReceiveBeginPlay`)
  (`self.EnableMouseEvents` false))

(event `EnableMouseEvents`
  (params (NewEnable :type Boolean))
  (bind _returnvalue (`GameplayStatics.GetPlayerController` 0))
  (`/Engine/EditorBlueprintResources/StandardMacros.IsValid` _returnvalue
    (:`Is Valid`
      (set `PlayerController.bEnableMouseOverEvents` NewEnable _returnvalue))))

(event `self.Sphere.OnBeginCursorOver`
  (params (TouchedComponent :type "PrimitiveComponent Object Reference"))
  (bind _ghostball (`self.GhostBall`))
  (`/Engine/EditorBlueprintResources/StandardMacros.IsValid` _ghostball :!label _label
    (:`Is Valid`
      (`/Game/Blueprints/Chakras/BP_ChakraBall_Base.SetColor` _ghostball (`self.HoveringColor`))
      (`self.UpdateInteractPrompt` true))))

(event `AddGhostChakra`
  ;[1 1 1] Add a ghost chakra if the player has the right chakra
  (`self.AddChakra` (`SceneComponent.K2_GetComponentToWorld` (`self.Sphere`)) (`self.ChakraMaterial`) true))

(event `Set Can Interact`
  (params (NewCanInteract :type Boolean))
  (bind _ghostball (`self.GhostBall`))
  (if NewCanInteract
    (goto _label)
    (else
      (`/Engine/EditorBlueprintResources/StandardMacros.IsValid` _ghostball :!label _label_2
        (:`Is Valid`
          (`/Game/Blueprints/Chakras/BP_ChakraBall_Base.SetColor` _ghostball (`self.GhostColor`))
          (`self.UpdateInteractPrompt` false))))))

(event `self.Sphere.OnEndCursorOver`
  (params (TouchedComponent :type "PrimitiveComponent Object Reference"))
  (goto _label_2))

(event `self.InteractEvent`
  (bind _powerstand (`self.PowerStand`))
  ;[1 1 1] Adds a definitive chakra
  (`self.DeleteGhostChakra`)
  (`self.AddChakra` (`SceneComponent.K2_GetComponentToWorld` (`self.Sphere`)) (`self.ChakraMaterial`))
  (`PrimitiveComponent.SetCollisionEnabled` (`self.Sphere`) "NoCollision")
  (bind _asfirst_person_character (cast `/Game/FirstPerson/Player/FirstPersonCharacter` (`GameplayStatics.GetPlayerPawn` 0)))
  (bind _chakrasinventory (`/Game/FirstPerson/Player/FirstPersonCharacter.ChakrasInventory` _asfirst_person_character))
  ;[1 1 1] Remove the chakra from the player's inventory
  (for (_array_element _array_index) _chakrasinventory
    (if (`|EnumEquality` _array_element (`self.ChakraName`))
      (`KismetArrayLibrary.Array_Remove` _chakrasinventory _array_index)
      (break)))
  ;[1 1 1] Spawn a power if it must
  (`/Engine/EditorBlueprintResources/StandardMacros.IsValid` _powerstand
    (:`Is Valid`
      (`/Game/Blueprints/Powers/Pickables/BP_Stand.SpawnPower` _powerstand (`self.RelatedPower`)))
    (:`Is Not Valid`
      ;[1 1 1] Ends the game if it must
      (if (`self.IsEnd`)
        (bind _asfirst_person_character_2 (cast `/Game/FirstPerson/Player/FirstPersonCharacter` (`GameplayStatics.GetPlayerPawn` 0)))
        (bind _uimanager (`/Game/FirstPerson/Player/FirstPersonCharacter.UIManager` _asfirst_person_character_2))
        (`/Engine/EditorBlueprintResources/StandardMacros.IsValid` _uimanager
          (:`Is Valid`
            (`/Game/Blueprints/UI/UiManager.EndGame` _uimanager))
          (:`Is Not Valid`
            (bind _returnvalue (`GameplayStatics.GetActorOfClass` "/Game/Blueprints/UI/UiManager.UiManager_C"))
            (`/Game/Blueprints/UI/UiManager.EndGame` _returnvalue)))))))

(fn `AddChakra`
  (params (SpawnTransform :type "Transform Structure") (ChakraMaterial :type "MaterialInstance Object Reference") (IsGhost :type Boolean))
  (bind _returnvalue (`|SpawnActorFromClass` "/Game/Blueprints/Chakras/BP_ChakraBall_Base.BP_ChakraBall_Base_C" SpawnTransform "Undefined" "OverrideRootScale" null null))
  (`/Game/Blueprints/Chakras/BP_ChakraBall_Base.ResetMaterial` _returnvalue ChakraMaterial)
  (if IsGhost
    (set `self.GhostBall` _returnvalue)
    (`self.EnableMouseEvents` true)
    (`/Game/Blueprints/Chakras/BP_ChakraBall_Base.SetColor` _returnvalue (`self.GhostColor`))
    (else
      (set `self.Found` false))))

(fn `DeleteGhostChakra`
  (`/Engine/EditorBlueprintResources/StandardMacros.IsValid` (`self.GhostBall`)
    (:`Is Valid`
      (`self.K2_DestroyActor` (`self.GhostBall`))
      (set `self.GhostBall` null)
      (set `self.Found` false)
      (`self.UpdateInteractPrompt` false))))

(fn `UserConstructionScript`)