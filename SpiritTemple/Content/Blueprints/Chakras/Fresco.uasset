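; Fresco puzzle actor that plays a level sequence once enough chakras have been placed in its linked holders.
; At construction it registers itself with each chakra holder and sets its counter to the number of holders.
; Each PlacedChakra event decrements the counter, and the sequence plays once, guarded by a flag, when the check finds one or fewer left.
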(event `PlacedChakra`
  (bind _result (`/Engine/EditorBlueprintResources/StandardMacros.DecrementInt` (`self.ChakrasCount`))
    (:`  `
      (if (and (<= _result 1) (not (`self.SequenceFlag`)))
        (set `self.SequenceFlag` true)
        (`MovieSceneSequencePlayer.Play` (`LevelSequenceActor.SequencePlayer` (`self.Sequence`)))))))

(fn `UserConstructionScript`
  (bind _chakraholders (`self.ChakraHolders`))
  (for _array_element _chakraholders
    (set `/Game/Blueprints/Chakras/BP_ChakraHolder_Base.Fresco` self _array_element))
  (set `self.ChakrasCount` (`KismetArrayLibrary.Array_Length` _chakraholders)))