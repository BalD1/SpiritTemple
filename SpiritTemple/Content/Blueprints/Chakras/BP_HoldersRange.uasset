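; BP_HoldersRange is a proximity trigger that gates interaction with a set of chakra holders.
; When the FirstPersonCharacter enters the Trigger volume, it enables mouse events on every holder in the ChakraHolders array.
; On exit it clears the character's interact prompt, then turns off each holder's interactability and mouse events.
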(event `self.Trigger.OnComponentBeginOverlap`
  (params (OverlappedComponent :type "PrimitiveComponent Object Reference") (OtherActor :type "Actor Object Reference") (OtherComp :type "PrimitiveComponent Object Reference") (OtherBodyIndex :type Integer) (bFromSweep :type Boolean) (SweepResult :type "HitResult Structure (by ref)"))
  (cast `/Game/FirstPerson/Player/FirstPersonCharacter` OtherActor)
  (for _array_element (`self.ChakraHolders`)
    (`/Game/Blueprints/Chakras/BP_ChakraHolder_Base.EnableMouseEvents` _array_element true)))

(event `self.Trigger.OnComponentEndOverlap`
  (params (OverlappedComponent :type "PrimitiveComponent Object Reference") (OtherActor :type "Actor Object Reference") (OtherComp :type "PrimitiveComponent Object Reference") (OtherBodyIndex :type Integer))
  (bind _asfirst_person_character (cast `/Game/FirstPerson/Player/FirstPersonCharacter` OtherActor))
  (`/Game/FirstPerson/Player/FirstPersonCharacter.CanInteractEvent` _asfirst_person_character false "")
  (for _array_element (`self.ChakraHolders`)
    (`/Game/Blueprints/Chakras/BP_ChakraHolder_Base.Set Can Interact` _array_element false)
    (`/Game/Blueprints/Chakras/BP_ChakraHolder_Base.EnableMouseEvents` _array_element false)))

(fn `UserConstructionScript`)