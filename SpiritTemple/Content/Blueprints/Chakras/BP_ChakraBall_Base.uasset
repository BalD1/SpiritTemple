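; Base Blueprint for a chakra ball that spins its sphere and, when flagged as an item, acts as a pickup.
; Player overlap with the trigger adds the chakra by name to the FirstPersonCharacter and destroys the ball.
; Non-item balls have trigger collision disabled, and helper functions switch the item state or reapply the chakra and glass materials.
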(event `self.ReceiveBeginPlay`
  (`PrimitiveComponent.SetMaterial` (`self.Chakra`) 0 (`self.ChakraMaterial`))
  (if (not (`self.IsItem`))
    (`PrimitiveComponent.SetCollisionEnabled` (`self.Trigger`) "NoCollision")))

(event `self.ReceiveTick`
  (params (DeltaSeconds :type "Float (single-precision)"))
  (bind (_returnvalue_roll _returnvalue_pitch _returnvalue_yaw) (`KismetMathLibrary.BreakRotator` (`SceneComponent.K2_GetComponentRotation` (`self.Sphere`))))
  (`SceneComponent.K2_SetWorldRotation` (`self.Sphere`) (`KismetMathLibrary.MakeRotator` _returnvalue_roll _returnvalue_pitch (+ _returnvalue_yaw (* DeltaSeconds (`self.RotationSpeed`)))) false false))

(event `self.Trigger.OnComponentBeginOverlap`
  (params (OverlappedComponent :type "PrimitiveComponent Object Reference") (OtherActor :type "Actor Object Reference") (OtherComp :type "PrimitiveComponent Object Reference") (OtherBodyIndex :type Integer) (bFromSweep :type Boolean) (SweepResult :type "HitResult Structure (by ref)"))
  (if (`self.IsItem`)
    (bind _asfirst_person_character (cast `/Game/FirstPerson/Player/FirstPersonCharacter` OtherActor))
    (`/Game/FirstPerson/Player/FirstPersonCharacter.AddChakra` _asfirst_person_character (`self.Name`))
    (`self.K2_DestroyActor`)))

(fn `ResetIsItem`
  (params (NewIsItem :type Boolean))
  (bind _trigger (`self.Trigger`))
  (set `self.IsItem` NewIsItem)
  (if (`self.IsItem`)
    (`PrimitiveComponent.SetCollisionEnabled` _trigger "QueryOnly")
    (else
      (`PrimitiveComponent.SetCollisionEnabled` _trigger "NoCollision"))))

(fn `ResetMaterial`
  (params (`NewMaterial?` :type "MaterialInstance Object Reference"))
  (`/Engine/EditorBlueprintResources/StandardMacros.IsValid` `NewMaterial?`
    (:`Is Valid`
      (set `self.ChakraMaterial` `NewMaterial?`))
    (:`Is Not Valid`
      _))
  (`PrimitiveComponent.SetMaterial` (`self.Chakra`) 0 (`self.ChakraMaterial`))
  (`PrimitiveComponent.SetMaterial` (`self.Sphere`) 0 "/Game/StarterContent/Materials/M_Glass.M_Glass"))

(fn `UserConstructionScript`)