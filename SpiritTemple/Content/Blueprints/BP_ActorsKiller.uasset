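; BP_ActorsKiller is a one-shot trigger actor that destroys every actor in its ActorsToKill list, then itself, when the FirstPersonCharacter overlaps its Trigger component.
; The UseTrigger event flip-flops the Trigger's collision between disabled and query-only, starting with disabled.
; Each toggle also recolors the TriggerState text (green when disabled, red when enabled) and prints the flip-flop's boolean in it.
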(event `UseTrigger`
  (bind _triggerstate (`self.TriggerState`))
  (bind _isa (`/Engine/EditorBlueprintResources/StandardMacros.FlipFlop`)
    (:`A`
      (`PrimitiveComponent.SetCollisionEnabled` (`self.Trigger`) "NoCollision")
      (`TextRenderComponent.SetTextRenderColor` _triggerstate (`KismetMathLibrary.Conv_LinearColorToColor` (struct :`G` 1.0 :`A` 1.0))))
    (:`B`
      (`PrimitiveComponent.SetCollisionEnabled` (`self.Trigger`) "QueryOnly")
      (`TextRenderComponent.SetTextRenderColor` _triggerstate (`KismetMathLibrary.Conv_LinearColorToColor` (struct :`R` 1.0 :`A` 1.0)))))
  (`TextRenderComponent.K2_SetText` _triggerstate (`KismetTextLibrary.Conv_StringToText` (`KismetStringLibrary.Concat_StrStr` "Trigger is " (`KismetStringLibrary.Conv_BoolToString` _isa)))))

(event `KillsActors`
  (for _array_element (`self.ActorsToKill`)
    (`self.K2_DestroyActor` _array_element))
  (`self.K2_DestroyActor`))

(event `self.Trigger.OnComponentBeginOverlap`
  (params (OverlappedComponent :type "PrimitiveComponent Object Reference") (OtherActor :type "Actor Object Reference") (OtherComp :type "PrimitiveComponent Object Reference") (OtherBodyIndex :type Integer) (bFromSweep :type Boolean) (SweepResult :type "HitResult Structure (by ref)"))
  (cast `/Game/FirstPerson/Player/FirstPersonCharacter` OtherActor)
  (`self.KillsActors`))

(fn `UserConstructionScript`)